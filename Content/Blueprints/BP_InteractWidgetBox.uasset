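; Trigger box actor that shows on-screen or in-world instruction widgets for a door while the player is nearby.
; Box begin and end overlap events filter for the FirstPersonCharacter through a cast, then show or hide both InteractWidget and InstructionsWidget.
; It only toggles visibility and contains no door interaction or construction logic.
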(event OnComponentBeginOverlap(Box)
  (params (OverlappedComponent :type Primitive%20Component%20Object%20Reference) (OtherActor :type Actor%20Object%20Reference) (OtherComp :type Primitive%20Component%20Object%20Reference) (OtherBodyIndex :type Integer) (bFromSweep :type Boolean) (SweepResult :type Hit%20Result%20Structure%20%28by%20ref%29))
  ;[1 1 1] Box Overlap Events to display widget instructions for door.
  (Utilities|Casting|CastToFirstPersonCharacter OtherActor)
  (Rendering|SetVisibility (Variables|Default|GetInteractWidget) true false)
  (Rendering|SetVisibility (Variables|Default|GetInstructionsWidget) true false))

(event OnComponentEndOverlap(Box)
  (params (OverlappedComponent :type Primitive%20Component%20Object%20Reference) (OtherActor :type Actor%20Object%20Reference) (OtherComp :type Primitive%20Component%20Object%20Reference) (OtherBodyIndex :type Integer))
  ;[1 1 1] Box Overlap Events to display widget instructions for door.
  (Utilities|Casting|CastToFirstPersonCharacter OtherActor)
  (Rendering|SetVisibility (Variables|Default|GetInteractWidget) false false)
  (Rendering|SetVisibility (Variables|Default|GetInstructionsWidget) false false))

(fn ConstructionScript)