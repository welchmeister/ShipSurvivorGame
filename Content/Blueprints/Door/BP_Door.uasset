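; BP_Door is an interactable door that swings open and closed on a timeline, or starts lockpicking when locked.
; Interaction matches the hit actor by display name, then toggles the door behind a DoOnce that resets when the timeline finishes.
; If locked, it shakes with a sound and, given a lockpick in the player's inventory, spawns a single far-off BP_Lockpicking_Actor with its widget.
; Box overlap shows prompt widgets while locked.
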(event OnComponentBeginOverlap(Box)
  (params (OverlappedComponent :type Primitive%20Component%20Object%20Reference) (OtherActor :type Actor%20Object%20Reference) (OtherComp :type Primitive%20Component%20Object%20Reference) (OtherBodyIndex :type Integer) (bFromSweep :type Boolean) (SweepResult :type Hit%20Result%20Structure%20%28by%20ref%29))
  ;[1 1 1] Box Overlap events
  (if (Variables|Default|GetIsLocked)
    (Utilities|Casting|CastToFirstPersonCharacter OtherActor)
    (Rendering|SetVisibility (Variables|Default|GetInteractWidget) true false)
    (Rendering|SetVisibility (Variables|Default|GetInstructionsWidget) true false)
    (else
      (Rendering|SetVisibility (Variables|Default|GetInteractWidget) false false)
      (Rendering|SetVisibility (Variables|Default|GetInstructionsWidget) false false))))

(event OnComponentEndOverlap(Box)
  (params (OverlappedComponent :type Primitive%20Component%20Object%20Reference) (OtherActor :type Actor%20Object%20Reference) (OtherComp :type Primitive%20Component%20Object%20Reference) (OtherBodyIndex :type Integer))
  ;[1 1 1] Box Overlap events
  (Utilities|Casting|CastToFirstPersonCharacter OtherActor)
  (Rendering|SetVisibility (Variables|Default|GetInteractWidget) false false)
  (Rendering|SetVisibility (Variables|Default|GetInstructionsWidget) false false))

(event Custom|UseDoor
  ;[1 1 1] Opens & closes door.
  (Utilities|FlowControl|DoOnce false
    (:Completed
      (if (not (Variables|Default|GetIsOpen))
        (Variables|Default|SetIsOpen true)
        (bind _door (Timeline|Door%20Timeline Play)
          (:Update
            (Transformation|SetRelativeRotation (Variables|Default|GetDoor) (Math|Rotator|MakeRotator 0.0 0.0 (Math|Float|Lerp 0.0 1e+02 _door)) false false))
          (:Finished
            (CallFunction|ResetDoorOpening)))
        (else
          (Variables|Default|SetIsOpen false)
          (Timeline|Door%20Timeline Reverse))))))

(event Custom|CreateLock
  ;[1 1 1] Creates the lockpicking actor & widget.
  (if (CallFunction|AnyLockpicks)
    (bind _returnvalue (Actor|GetActorOfClass "/Game/Blueprints/Puzzles/Lockpicking/BP_Lockpicking_Actor.BP_Lockpicking_Actor_C"))
    (Utilities|IsValid _returnvalue
      (:Is%20Not%20Valid
        (bind _returnvalue_2 (Game|SpawnActorfromClass "/Game/Blueprints/Puzzles/Lockpicking/BP_Lockpicking_Actor.BP_Lockpicking_Actor_C" (Math|Transform|MakeTransform "0.000000,0.000000,1000000.000000" "0, 0, 0" "1.000000,1.000000,1.000000") "Undefined" "MultiplyWithRoot" 0 self 0))
        (Default|CreateLockpickingWidget _returnvalue_2)))))

(event Custom|ResetDoorOpening
  ;[1 1 1] Opens & closes door.
  (Utilities|FlowControl|DoOnce false) ; enters at Reset
)

(event Custom|ShakeDoor
  ;[1 1 1] Door Shake
  (Audio|PlaySoundatLocation "/Game/Meshes/PuzzleMeshes/Audio/DoorsAndFurnitures/Lock02.Lock02" (Transformation|GetActorLocation) "0, 0, 0" 1.0 1.0 0.0 0 0 0 0)
  (Utilities|FlowControl|FlipFlop
    (:A
      (bind _alpha (Timeline|Timeline PlayFromStart)
        (:Update
          (Transformation|SetRelativeRotation (Variables|Default|GetDoor) (Math|Rotator|MakeRotator 0.0 0.0 _alpha) false false))))
    (:B
      (Timeline|Timeline ReverseFromEnd))))

(event EventInteraction
  (params (Character :type First%20Person%20Character%20Object%20Reference) (HitActor :type Primitive%20Component%20Object%20Reference))
  ;[1 1 1] On interact with.
  (if (Utilities|Enum|Equal(Enum) (Utilities|GetDisplayName HitActor) "BP_Door.Door SM_Door")
    (if (not (Variables|Default|GetIsLocked))
      (CallFunction|UseDoor)
      (else
        (CallFunction|ShakeDoor)
        (CallFunction|CreateLock)))))

(fn ConstructionScript)

(fn AnyLockpicks
  (if (Utilities|Array|ContainsItem (Variables|/Game/Blueprints/Inventory/ActorComponents/AC_Inventory.AC_Inventory_C|GetSlots (Variables|/Game/FirstPerson/FPSword/Blueprints/FirstPersonCharacter.FirstPersonCharacter_C|GetAC_Inventory (CallFunction|GetPlayer))) "lockpick")
    (return true)
    (else
      (return false))))