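; BP_DialogueBox is an interactable actor that runs a dialogue with the first-person player and shows a widget while they stand in its trigger box.
; Interaction blends the camera to this actor, disables player movement, switches to game-and-UI input and calls Speech on its BPCDialogue component.
; DialogueComplete blends the view back to the player and restores walking, look input and game-only input.
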(event OnComponentBeginOverlap(Box)
  (params (OverlappedComponent :type Primitive%20Component%20Object%20Reference) (OtherActor :type Actor%20Object%20Reference) (OtherComp :type Primitive%20Component%20Object%20Reference) (OtherBodyIndex :type Integer) (bFromSweep :type Boolean) (SweepResult :type Hit%20Result%20Structure%20%28by%20ref%29))
  (Utilities|Casting|CastToFirstPersonCharacter OtherActor)
  (Rendering|SetVisibility (Variables|Default|GetWidget) true false))

(event OnComponentEndOverlap(Box)
  (params (OverlappedComponent :type Primitive%20Component%20Object%20Reference) (OtherActor :type Actor%20Object%20Reference) (OtherComp :type Primitive%20Component%20Object%20Reference) (OtherBodyIndex :type Integer))
  (Utilities|Casting|CastToFirstPersonCharacter OtherActor)
  (Rendering|SetVisibility (Variables|Default|GetWidget) false false))

(event Custom|DialogueComplete
  (bind _returnvalue (Game|GetPlayerController 0))
  ;[1 1 1] Interaction
  (Game|Player|SetViewTargetwithBlend (Game|GetPlayerController 0) (Variables|Default|GetPlayerRef) 0.5 "VTBlend_Linear" 0.0 false)
  (Pawn|Components|CharacterMovement|SetMovementMode (Variables|/Script/Engine.Character|GetCharacterMovement (Variables|Default|GetPlayerRef)) "MOVE_Walking" 0)
  (Input|ResetIgnoreLookInput _returnvalue)
  (Input|SetIgnoreLookInput _returnvalue false)
  (Input|SetInputModeGameOnly _returnvalue false))

(event EventBeginPlay
  (bind _asfirst_person_character (Utilities|Casting|CastToFirstPersonCharacter (Game|GetPlayerCharacter 0)))
  (Variables|Default|SetPlayerRef _asfirst_person_character))

(event EventInteraction
  (params (Character :type Actor%20Object%20Reference))
  (bind _returnvalue (Game|GetPlayerController 0))
  ;[1 1 1] Interaction
  (Game|Player|SetViewTargetwithBlend _returnvalue self 0.5 "VTBlend_Linear" 0.0 false)
  (Pawn|Components|CharacterMovement|DisableMovement (Variables|/Script/Engine.Character|GetCharacterMovement (Variables|Default|GetPlayerRef)))
  (Input|SetInputModeGameandUI _returnvalue 0 "LockAlways" true false)
  (Default|Speech (Variables|Default|GetBPC_Dialogue)))

(fn ConstructionScript)