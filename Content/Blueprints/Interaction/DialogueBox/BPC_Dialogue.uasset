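; Dialogue component that steps through an array of text lines for a named speaker in a dialogue box.
; On BeginPlay it creates a W_Dialogue widget with name and text colors.
; Each Speech call sends the current line, name and text delay to the widget, then advances the index.
; Once the index runs past the last line, it resets, clears the widget and notifies its BP_DialogueBox owner that dialogue is complete.
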(event Custom|Speech
  (bind _dialogue (Variables|Default|GetDialogue))
  ;[1 1 1] Display Dialogue and clear screen when no dialogue to show.
  (Default|IncomingText (Variables|Default|GetW_DialogueRef) (Utilities|Array|Get(acopy) _dialogue (Variables|Default|GetCurrentDialogue)) (Variables|Default|GetTextDelay) (Variables|Default|GetName))
  (bind _result (Math|Integer|IncrementInt (Variables|Default|GetCurrentDialogue))
    (:%20%20
      (if (>= _result (+ (Utilities|Array|Length _dialogue) 1))
        (Variables|Default|SetCurrentDialogue 0)
        (Default|ClearScreen (Variables|Default|GetW_DialogueRef))
        (bind _asbp_dialogue_box (Utilities|Casting|CastToBP_DialogueBox (Components|GetOwner)))
        (Default|DialogueComplete _asbp_dialogue_box)))))

(event EventBeginPlay
  ;[1 1 1] BeginPlay
  (bind _returnvalue (UserInterface|CreateWidget "/Game/Blueprints/Widgets/W_Dialogue.W_Dialogue_C" 0 (Variables|Default|GetName%20Color) (Variables|Default|GetDialogue%20Color)))
  (Variables|Default|SetW_DialogueRef _returnvalue))