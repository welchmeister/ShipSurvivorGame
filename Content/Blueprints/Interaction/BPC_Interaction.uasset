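; Interaction component that detects interactable actors in front of its owner and lets input trigger them.
; On BeginPlay it creates the interact message widget and starts a looping timer that sphere-traces forward from the owner.
; Hit actors implementing BPI_Interaction become the target; otherwise the target and widget text are cleared.
; The IA_Interaction input calls InteractionMessage on the current valid target.
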(event Custom|BeginTrace
  ;[1 1 1] Starts & updates interaction trace.
  (Utilities|Time|SetTimerbyEvent (delegate Custom|UpdateTrace) 0.2 true))

(event Custom|UpdateTrace
  ;[1 1 1] Starts & updates interaction trace.
  (CallFunction|InteractionTrace))

(event Input|EnhancedActionEvents|EnhancedInputActionIA_Interaction
  (params (ActionValue :type Boolean) (ElapsedSeconds :type Float%20%28double-precision%29) (TriggeredSeconds :type Float%20%28double-precision%29) (InputAction :type Input%20Action%20Object%20Reference :default "/Game/FirstPerson/Input/Actions/IA_Interaction.IA_Interaction"))
  ;[1 1 1] Allows to interact.
  (:Started
    (bind _targetactor (Variables|Default|GetTargetActor)
      (:then
        (Class|BPIInteraction|Interaction(Message) _targetactor))
      (:else))))

(event EventBeginPlay
  ;[1 1 1] Creates widget & trace.
  (CallFunction|CreateInteractMessage)
  (CallFunction|BeginTrace))

(fn InteractionTrace
  (bind _returnvalue (Components|GetOwner))
  (bind _returnvalue_2 (Transformation|GetActorLocation _returnvalue))
  ;[1 1 1] Creates the interaction trace & interaction message if target is valid.
  (bind (_outhit _returnvalue_3) (Collision|SphereTraceByChannel _returnvalue_2 (+ _returnvalue_2 (* (Transformation|GetActorForwardVector _returnvalue) 1e+02)) 5e+01 "TraceTypeQuery3" false 0 "None"))
  (if _returnvalue_3
    (if (Utilities|DoesObjectImplementInterface (.HitActor (Collision|BreakHitResult _outhit)) "/Game/Blueprints/Interfaces/BPI_Interaction.BPI_Interaction_C")
      (Variables|Default|SetTargetActor (.HitActor (Collision|BreakHitResult _outhit)))
      (else
        (Variables|Default|SetTargetActor 0)
        (Default|SetMessage (Variables|Default|GetWB_InteractMessage))))
    (else
      (Variables|Default|SetTargetActor 0)
      (Default|SetMessage (Variables|Default|GetWB_InteractMessage)))))

(fn CreateInteractMessage
  ;[1 1 1] Creates the interact widget.
  (bind _returnvalue (UserInterface|CreateWidget "/Game/Blueprints/Interaction/UI/WB_InteractMessage.WB_InteractMessage_C"))
  (bind _output_get (Variables|Default|SetWB_InteractMessage _returnvalue))
  (UserInterface|Viewport|AddtoViewport _output_get 0))