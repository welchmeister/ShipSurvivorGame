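; Game mode for Level 1 that runs the level's HUD widgets, collectable count and pressure-plate door puzzle.
; On BeginPlay it shows the timer, counts BP_Collectables actors, binds plate up/down events and finds BP_Door6.
; Plate events track pressed plates, unlocking the door at the completion count and relocking it on any release.
; Separate events add and remove the collectables widget; a never-reset flag allows only one creation.
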(event Custom|PressurePlateDown
  (bind _door (Variables|Default|GetDoor))
  (bind _result (Math|Integer|IncrementInt (Variables|Default|GetPressurePlatesDown))
    (:%20%20
      (bind _output_get (Variables|Default|SetPressurePlatesDown _result))
      (if (== _output_get (Variables|Default|GetPressurePlatesForCompletion))
        (Variables|/Game/Blueprints/Puzzles/Doors/BP_Door6.BP_Door6_C|SetLocked? _door false)
        (Variables|/Game/Blueprints/Puzzles/Doors/BP_Door6.BP_Door6_C|SetDoorClosed? _door true)
        (Default|DoorUnlock (Variables|Default|GetDoor))))))

(event Custom|PressurePlateUp
  (bind _result (Math|Integer|DecrementInt (Variables|Default|GetPressurePlatesDown))
    (:%20%20
      (Variables|Default|SetPressurePlatesDown _result)
      (Variables|/Game/Blueprints/Puzzles/Doors/BP_Door6.BP_Door6_C|SetLocked? (Variables|Default|GetDoor) true))))

(event Custom|Add%20Collectable%20Items%20Widget
  (if (not (Variables|Default|GetIsCollectableWidgetActivated?%20))
    (Variables|Default|SetIsCollectableWidgetActivated?%20 true)
    (bind _returnvalue (UserInterface|CreateWidget "/Game/Blueprints/Widgets/W_Collectables.W_Collectables_C" (Game|GetPlayerController 0)))
    (bind _output_get (Variables|Default|SetCollectables%20Widget _returnvalue))
    (UserInterface|Viewport|AddtoViewport _output_get 0)))

(event Custom|Remove%20Collectable%20Items%20Widget
  (Widget|RemovefromParent (Variables|Default|GetCollectables%20Widget)))

(event EventBeginPlay
  (bind _returnvalue (UserInterface|CreateWidget "/Game/Blueprints/Widgets/W_Timer.W_Timer_C"))
  (bind _output_get (Variables|Default|SetTimer _returnvalue))
  (UserInterface|Viewport|AddtoViewport _output_get 0)
  (bind _outactors (Actor|GetAllActorsOfClass "/Game/Blueprints/Puzzles/Collectables/BP_Collectables.BP_Collectables_C"))
  (bind _output_get_2 (Variables|Default|SetCollectables%20Left (Utilities|Array|Length _outactors)))
  (Variables|Default|SetTotal%20Collectables _output_get_2)
  (EventDispatchers|BindEventtoOnPressurePlateDown (delegate Custom|PressurePlateDown))
  (EventDispatchers|BindEventtoOnPressPlateUp (delegate Custom|PressurePlateUp))
  (bind _returnvalue_2 (Actor|GetActorOfClass "/Game/Blueprints/Puzzles/Doors/BP_Door6.BP_Door6_C"))
  (Variables|Default|SetDoor _returnvalue_2))

(fn ConstructionScript)