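; BP_Drawer is an interactable drawer holding a configurable item mesh that can be inspected as a note.
; Interaction matches hard-coded display names of four instances: drawer hits toggle a timeline slide along local Y with sound, locked by DoOnce until finished.
; Note hits spawn an off-scene BP_InspectItem, passing mesh, description and note text.
; An older note-widget path is unconnected, though its IA_Back exit handler remains.
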(event Custom|ResetDrawer
  (bind _returnvalue (Transformation|GetActorLocation))
  (bind _drawer (Variables|Default|GetDrawer))
  (bind _drawer_2 (Variables|Default|GetDrawer))
  (bind _relativelocation (Variables|/Script/Engine.SceneComponent|GetRelativeLocation _drawer_2))
  (bind _relativelocation_2 (Variables|/Script/Engine.SceneComponent|GetRelativeLocation _drawer))
  ;[1 1 1] Interaction
  (Utilities|FlowControl|DoOnce false) ; enters at Reset
)

(event Input|EnhancedActionEvents|EnhancedInputActionIA_Back
  (params (ActionValue :type Boolean) (ElapsedSeconds :type Float%20%28double-precision%29) (TriggeredSeconds :type Float%20%28double-precision%29) (InputAction :type Input%20Action%20Object%20Reference :default "/Game/FirstPerson/Input/Actions/IA_Back.IA_Back"))
  (:Started
    ;[1 1 1] Exit Note Inspection
    (Utilities|IsValid (Variables|Default|GetNote)
      (:Is%20Valid
        ;[1 1 1] Interaction
        (Widget|RemovefromParent (Variables|Default|GetNote))
        (Variables|Default|SetNote 0)
        (Input|ResetIgnoreLookInput (Game|GetPlayerController 0))
        (Pawn|Components|CharacterMovement|SetMovementMode (Variables|/Script/Engine.Character|GetCharacterMovement (Game|GetPlayerCharacter 0)) "MOVE_Walking" 0)))))

(event EventInteraction
  (params (Character :type First%20Person%20Character%20Object%20Reference) (HitActor :type Primitive%20Component%20Object%20Reference))
  (bind _returnvalue (Transformation|GetActorLocation))
  (bind _drawer (Variables|Default|GetDrawer))
  (bind _drawer_2 (Variables|Default|GetDrawer))
  (bind _relativelocation (Variables|/Script/Engine.SceneComponent|GetRelativeLocation _drawer_2))
  (bind _relativelocation_2 (Variables|/Script/Engine.SceneComponent|GetRelativeLocation _drawer))
  ;[1 1 1] Interaction
  (switch string (Utilities|GetDisplayName HitActor)
    (:BP_Drawer3283.Drawer%20Drawer
      (if (Variables|Default|GetCanOpens?) :!label _label
        (Utilities|FlowControl|DoOnce false
          (:Completed
            (if (not (>= (.y (Variables|/Script/Engine.SceneComponent|GetRelativeLocation (Variables|Default|GetDrawer))) 25.0))
              (Audio|PlaySoundatLocation "/Game/Meshes/PuzzleMeshes/Audio/DoorsAndFurnitures/DrawerClose02.DrawerClose02" _returnvalue "0, 0, 0" 1.0 1.0 0.0 0 0 0 0)
              (Variables|Default|SetStartLocation (Math|Vector|MakeVector (.x _relativelocation) (.y _relativelocation) (.z _relativelocation)))
              (Variables|Default|SetEndLocation (Math|Vector|MakeVector (.x _relativelocation) (+ (.y _relativelocation) 3e+01) (.z _relativelocation)))
              (bind _open_drawer (Timeline|Timeline PlayFromStart)
                (:Update
                  (Transformation|SetRelativeLocation (Variables|Default|GetDrawer) (Math|Vector|Lerp(Vector) (Variables|Default|GetStartLocation) (Variables|Default|GetEndLocation) _open_drawer) false false))
                (:Finished
                  (Variables|Default|SetCanOpens? true)
                  (CallFunction|ResetDrawer)))
              (else
                (Audio|PlaySoundatLocation "/Game/Meshes/PuzzleMeshes/Audio/DoorsAndFurnitures/DrawerClose02.DrawerClose02" _returnvalue "0, 0, 0" 1.0 1.0 0.0 0 0 0 0)
                (Variables|Default|SetStartLocation (Math|Vector|MakeVector (.x _relativelocation_2) (.y _relativelocation_2) (.z _relativelocation_2)))
                (Variables|Default|SetEndLocation (Math|Vector|MakeVector (.x _relativelocation_2) (- (.y _relativelocation_2) 3e+01) (.z _relativelocation_2)))
                (bind _open_drawer_2 (Timeline|Timeline_0 PlayFromStart)
                  (:Update
                    (Transformation|SetRelativeLocation (Variables|Default|GetDrawer) (Math|Vector|Lerp(Vector) (Variables|Default|GetStartLocation) (Variables|Default|GetEndLocation) _open_drawer_2) false false))
                  (:Finished
                    (Variables|Default|SetCanOpens? true)
                    (CallFunction|ResetDrawer)))))))))
    (:BP_Drawer3283.Item%20Note
      (bind _returnvalue_2 (Game|SpawnActorfromClass "/Game/Blueprints/Interaction/Inspect/BP_InspectItem.BP_InspectItem_C" (Math|Transform|MakeTransform "0.000000,-2000.000000,100.000000") "Undefined" "MultiplyWithRoot" 0 0 :!label _label_2))
      (Default|SetInspectRotation _returnvalue_2 (Variables|Default|GetItem%20Inspection%20Rotation))
      (Default|SetInspectScale _returnvalue_2 (Variables|Default|GetItem%20Inspection%20Scale))
      (Class|BPIInteraction|Inspect(Message) _returnvalue_2 Character (Variables|/Script/Engine.StaticMeshComponent|GetStaticMesh (Variables|Default|GetItem)) (Variables|Default|GetItem%20Name) (Variables|Default|GetItem%20Description))
      (Class|BPIInteraction|ReadNote(Message) _returnvalue_2 Character (Variables|Default|GetNoteText)))
    (:BP_Drawer3282.Drawer%20Drawer
      (goto _label))
    (:BP_Drawer3281.Drawer%20Drawer
      (goto _label))
    (:BP_Drawer3280.Drawer%20Drawer
      (goto _label))
    (:BP_Drawer3282.Item%20Note
      (goto _label_2))
    (:BP_Drawer3281.Item%20Note
      (goto _label_2))
    (:BP_Drawer3280.Item%20Note
      (goto _label_2))))

(event EventBeginPlay
  (bind _item (Variables|Default|GetItem))
  ;[1 1 1] BeginPlay
  (Components|StaticMesh|SetStaticMesh _item (Variables|Default|GetStaticMeshItem))
  (Transformation|SetRelativeScale3D _item (Variables|Default|GetScale)))

(fn ConstructionScript
  (bind _item (Variables|Default|GetItem))
  (Components|StaticMesh|SetStaticMesh _item (Variables|Default|GetStaticMeshItem))
  (Transformation|SetRelativeScale3D _item (Variables|Default|GetScale)))