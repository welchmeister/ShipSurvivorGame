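; BP_Collectables is an interactable Level 1 puzzle item that counts toward unlocking BP_Door5.
; On BeginPlay it caches the door through GetActorOfClass.
; Each interaction decrements CollectablesLeft on GM_Level1, destroys the item and calls AddCollectableItemsWidget while any remain.
; When the count reaches zero, it instead unlocks the door, removes the collectable widget and destroys itself.
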(event EventInteraction
  (params (Character :type First%20Person%20Character%20Object%20Reference) (HitActor :type Primitive%20Component%20Object%20Reference))
  (bind _asgm_level_1 (Utilities|Casting|CastToGM_Level1 (Game|GetGameMode)))
  (bind _result (Math|Integer|DecrementInt (Variables|/Game/Blueprints/Gamemode/GM_Level1.GM_Level1_C|GetCollectables%20Left _asgm_level_1))
    (:%20%20
      (bind _output_get (Variables|/Game/Blueprints/Gamemode/GM_Level1.GM_Level1_C|SetCollectables%20Left _asgm_level_1 _result))
      (if (== _output_get 0)
        (Default|UnlockDoor (Variables|Default|GetDoor5))
        (Default|RemoveCollectableItemsWidget _asgm_level_1)
        (Actor|DestroyActor)
        (else
          (Actor|DestroyActor)
          (Default|AddCollectableItemsWidget _asgm_level_1))))))

(event EventBeginPlay
  (bind _returnvalue (Actor|GetActorOfClass "/Game/Blueprints/Puzzles/Doors/BP_Door5.BP_Door5_C"))
  (Variables|Default|SetDoor5 _returnvalue))

(fn ConstructionScript
  (|CallParentFunction))

(fn PickupItem
  (params (ID :type Name :default "None") (DropItem :type ST%20Inventory%20Item%20Structure))
  (return false))