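; BP_CombinationLock is a puzzle padlock that the player opens by matching three dials to a stored combination.
; On BeginPlay it spawns BP_Dial actors onto padlock sockets, and interacting blends the view to the lock, freezes the player and enables mouse-driven widget clicks.
; CheckEveryTurn compares dial numbers to the combination.
; A match animates the latch, then restores player control, signals puzzle completion and destroys the lock and dials.
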(event Custom|ExitView
  (bind _returnvalue (Game|GetPlayerController 0))
  (bind _returnvalue_2 (Game|GetPlayerCharacter 0))
  (bind _returnvalue_3 (Game|GetPlayerController 0))
  ;[1 1 1] Exit View of Puzzle
  (Game|Player|SetViewTargetwithBlend _returnvalue_3 _returnvalue_2 0.5 "VTBlend_Linear" 0.0 false)
  (Input|DisableInput _returnvalue_3 0)
  (Input|ResetIgnoreLookInput _returnvalue_3)
  (Variables|/Script/Engine.PlayerController|SetbShowMouseCursor _returnvalue_3 false)
  (Pawn|Components|CharacterMovement|SetMovementMode (Variables|/Script/Engine.Character|GetCharacterMovement _returnvalue_2) "MOVE_Walking" 0)
  (Input|ResetIgnoreLookInput _returnvalue)
  (Input|SetIgnoreLookInput _returnvalue false)
  (Input|SetInputModeGameOnly _returnvalue false))

(event Custom|CheckEveryTurn
  ;[1 1 1] Check Combination locks to see if correct
  (bind _local_success (CallFunction|CheckCode))
  (if _local_success
    (CallFunction|UnlockLock)))

(event Custom|UnlockLock
  ;[1 1 1] Unlock the Padlock
  (Audio|PlaySoundatLocation "/Game/Meshes/PuzzleMeshes/Audio/DoorsAndFurnitures/Unlock01.Unlock01" (Transformation|GetWorldLocation (Variables|Default|GetSM_Latch)) "0, 0, 0" 1.0 1.0 0.0 0 0 0 0)
  (bind _alpha (Timeline|Unlock_TL PlayFromStart)
    (:Update
      (Transformation|SetRelativeLocation (Variables|Default|GetSM_Latch) (Math|Vector|MakeVector 0.0 0.0 (Math|Float|Lerp 0.0 2.0 _alpha)) false false)
      (Utilities|FlowControl|Delay 1.0)
      (CallFunction|ExitView)
      (Default|CallOnPuzzleCompleted)
      (Actor|DestroyActor (Variables|Default|GetDials))
      (Actor|DestroyActor))))

(event Input|EnhancedActionEvents|EnhancedInputActionIA_Action
  (params (ActionValue :type Boolean) (ElapsedSeconds :type Float%20%28double-precision%29) (TriggeredSeconds :type Float%20%28double-precision%29) (InputAction :type Input%20Action%20Object%20Reference :default "/Game/FirstPerson/Input/Actions/IA_Action.IA_Action"))
  (bind _widgetinteraction (Variables|Default|GetWidgetInteraction))
  ;[1 1 1] Send line trace to hit widget button
  (:Started
    (Class|WidgetInteractionComponent|PressPointerKey _widgetinteraction "LeftMouseButton"))
  (:Completed
    (Class|WidgetInteractionComponent|ReleasePointerKey _widgetinteraction "LeftMouseButton")))

(event Input|EnhancedActionEvents|EnhancedInputActionIA_Back
  (params (ActionValue :type Boolean) (ElapsedSeconds :type Float%20%28double-precision%29) (TriggeredSeconds :type Float%20%28double-precision%29) (InputAction :type Input%20Action%20Object%20Reference :default "/Game/FirstPerson/Input/Actions/IA_Back.IA_Back"))
  ;[1 1 1] Exit View of Puzzle
  (:Started
    (CallFunction|ExitView)))

(event EventBeginPlay
  ;[1 1 1] BeginPlay
  (for _index (range 0 2)
    (bind _returnvalue (Game|SpawnActorfromClass "/Game/Blueprints/Puzzles/CombinationLock/BP_Dial.BP_Dial_C" (Math|Transform|MakeTransform "0, 0, 0" "0, 0, 0" "1.000000,1.000000,1.000000") "Undefined" "MultiplyWithRoot" 0 _index self 0))
    (Utilities|Array|Add (Variables|Default|GetDials) _returnvalue)
    (Transformation|AttachComponentToComponent _returnvalue (Variables|Default|GetSM_Combination_Padlock) (Utilities|Select :Index _index :Option%200 "Dial01" :Option%201 "Dial02" :Option%202 "Dial03") "KeepRelative" "KeepRelative" "KeepRelative" true)))

(event EventInteraction
  (params (Character :type First%20Person%20Character%20Object%20Reference) (HitActor :type Primitive%20Component%20Object%20Reference))
  (bind _returnvalue (Game|GetPlayerController 0))
  (bind _asfirst_person_character (CallFunction|GetPlayer))
  ;[1 1 1] Interaction
  (Game|Player|SetViewTargetwithBlend (Game|GetPlayerController 0) self 0.5 "VTBlend_Linear" 0.0 false)
  (Pawn|Components|CharacterMovement|DisableMovement (Variables|/Script/Engine.Character|GetCharacterMovement (Game|GetPlayerCharacter 0)))
  (Input|SetIgnoreLookInput _returnvalue true)
  (Utilities|FlowControl|Delay 0.5)
  (Input|EnableInput _returnvalue)
  (Variables|/Script/Engine.PlayerController|SetbShowMouseCursor _returnvalue true)
  (Input|SetInputModeGameandUI _returnvalue 0 "LockAlways" true false)
  (Default|Detach (Variables|/Game/FirstPerson/FPSword/Blueprints/FirstPersonCharacter.FirstPersonCharacter_C|GetAC_Inventory _asfirst_person_character))
  (Variables|/Game/FirstPerson/FPSword/Blueprints/FirstPersonCharacter.FirstPersonCharacter_C|SetOverlayState _asfirst_person_character "NewEnumerator4"))

(fn ConstructionScript)

(fn CheckCode
  (bind (_array_element _array_index) (Utilities|Array|ForEachLoopwithBreak (Variables|Default|GetDials) :!label _label)
    (:LoopBody
      (if (== (Variables|/Game/Blueprints/Puzzles/CombinationLock/BP_Dial.BP_Dial_C|GetNumber _array_element) (Utilities|Array|Get(acopy) (Variables|Default|GetLockCombination) _array_index))
        (LocalVariables|SetLocalSuccess true)
        (else
          (LocalVariables|SetLocalSuccess false)
          (goto _label Break))))
    (:Completed
      (return (LocalVariables|GetLocalSuccess)))))