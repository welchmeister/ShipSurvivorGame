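; Lockpicking minigame actor, shown through a scene capture and widget, that takes over player input and unlocks and uses a target door on success.
; Look input rotates the pick toward a random angle, and holding the lockpicking input tests it within an error margin.
; Looping timers turn, return or jiggle the lock.
; Jamming drains pick health until it snaps with a physics animation and is replaced, while the interaction input cancels.
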(event Custom|CreateLockpickingWidget
  (bind _returnvalue (Game|GetPlayerController 0))
  ;[1 1 1] Creates the lockpicking widget.
  (Rendering|SceneCapture|ShowOnlyActorComponents (Variables|Default|GetLockpicking_Capture) self false)
  (bind _returnvalue_2 (UserInterface|CreateWidget "/Game/Blueprints/Puzzles/Lockpicking/UI/WB_Lockpicking.WB_Lockpicking_C" 0 self))
  (bind _output_get (Variables|Default|SetWB_Lockpicking _returnvalue_2))
  (UserInterface|Viewport|AddtoViewport _output_get 0)
  (Input|DisableInput (CallFunction|GetPlayer) _returnvalue)
  (Input|EnableInput _returnvalue))

(event Custom|ForwardLockRotation
  ;[1 1 1] Forward lock rotation.
  (Utilities|Time|PauseTimerbyHandle (Variables|Default|GetBackwardLockTimer))
  (bind _returnvalue (Utilities|Time|SetTimerbyEvent (delegate Custom|UpdateForwardLockRotation) 0.02 true))
  (Variables|Default|SetForwardLockTimer _returnvalue)
  (Utilities|Time|PauseTimerbyHandle (Variables|Default|GetJammedLock)))

(event Custom|LockpickingSuccessful
  ;[1 1 1] Lockpicking successful.
  (Utilities|Time|SetTimerbyEvent (delegate Custom|LockpickingFinished) 0.5)
  (Variables|Default|SetLockComplete true))

(event Custom|LockpickingFinished
  (bind _returnvalue (Game|GetPlayerController 0))
  ;[1 1 1] Lockpicking successful.
  (Input|DisableInput _returnvalue)
  (Input|EnableInput (CallFunction|GetPlayer) _returnvalue)
  (bind _wb_lockpicking (Variables|Default|GetWB_Lockpicking)
    (:then
      (Widget|RemovefromParent _wb_lockpicking)
      (Utilities|IsValid (Variables|Default|GetWB_Lockpicking)
        (:Is%20Valid
          (Variables|Default|SetWB_Lockpicking 0)
          (bind _targetdoor (Variables|Default|GetTargetDoor)
            (:then
              (Default|UseDoor _targetdoor)
              (Variables|/Game/Blueprints/Door/BP_Door.BP_Door_C|SetIsLocked _targetdoor false))
            (:else)))))
    (:else)))

(event Custom|NewLockpick
  ;[1 1 1] Add new lockpick.
  (Utilities|Time|SetTimerbyEvent (delegate Custom|AddNewLockpick) 1.0)
  (Variables|Default|SetIsLockRotating false)
  (Input|DisableInput (Game|GetPlayerController 0)))

(event Custom|AddNewLockpick
  ;[1 1 1] Add new lockpick.
  (Rendering|SetVisibility (Variables|Default|GetLockpick) true false)
  (Rendering|SetVisibility (Variables|Default|GetLockpick_Broken1) false false)
  (Variables|Default|SetLockpickHealth 1e+02)
  (CallFunction|ResetLockpick)
  (Input|EnableInput (Game|GetPlayerController 0)))

(event Custom|LockpickAnim
  (bind _lockpick_broken2 (Variables|Default|GetLockpick_Broken2))
  ;[1 1 1] Lockpick animation.
  (Rendering|SetVisibility (Variables|Default|GetLockpick_Broken2) true false)
  (Rendering|SetVisibility (Variables|Default|GetLockpick) false false)
  (Physics|SetSimulatePhysics _lockpick_broken2 false)
  (Collision|SetCollisionEnabled _lockpick_broken2 "NoCollision")
  (Transformation|SetRelativeTransform (Variables|Default|GetLockpick_Broken2) (Transformation|GetRelativeTransform (Variables|Default|GetLockpick_Broken1)) false false)
  (Utilities|Time|SetTimerbyEvent (delegate Custom|BeginAnimation) 0.1))

(event Custom|BeginAnimation
  (bind _lockpick_broken2 (Variables|Default|GetLockpick_Broken2))
  (bind _lockpick_broken2_2 (Variables|Default|GetLockpick_Broken2))
  ;[1 1 1] Lockpick animation.
  (Physics|SetSimulatePhysics _lockpick_broken2 true)
  (Collision|SetCollisionEnabled _lockpick_broken2 "QueryAndPhysics")
  (Utilities|FlowControl|Delay 1.0)
  (Physics|SetSimulatePhysics _lockpick_broken2_2 false)
  (Collision|SetCollisionEnabled _lockpick_broken2_2 "NoCollision"))

(event Custom|UpdateBackwardLockRotation
  (bind _returnvalue (+ 0.0 6.0))
  (bind _lockrotation_scene (Variables|Default|GetLockRotation_Scene))
  (bind _relativerotation (Variables|/Script/Engine.SceneComponent|GetRelativeRotation _lockrotation_scene))
  (bind _returnvalue_2 (Math|Rotator|CombineRotators _relativerotation (Math|Rotator|MakeRotator _returnvalue 0.0 0.0)))
  ;[1 1 1] Backward lock rotation.
  (if (not (Variables|Default|GetIsLockRotating))
    (bind _output_get (Variables|Default|SetLockRotation (Math|Float|Clamp(Float) (.roll _returnvalue_2) -9e+01 0.0)))
    (Transformation|SetRelativeRotation (Variables|Default|GetLockRotation_Scene) (Math|Rotator|MakeRotator _output_get (.pitch _returnvalue_2) (.yaw _returnvalue_2)) false false)
    (CallFunction|LockpickBackward)
    (if (== (Variables|Default|GetLockRotation) 0.0)
      (Utilities|Time|PauseTimerbyHandle (Variables|Default|GetBackwardLockTimer)))))

(event Custom|BackwardLockRotation
  ;[1 1 1] Backward lock rotation.
  (Utilities|Time|PauseTimerbyHandle (Variables|Default|GetForwardLockTimer))
  (bind _returnvalue (Utilities|Time|SetTimerbyEvent (delegate Custom|UpdateBackwardLockRotation) 0.02 true))
  (Variables|Default|SetBackwardLockTimer _returnvalue))

(event Custom|UpdateForwardLockRotation
  (bind _returnvalue (- 0.0 3.0))
  (bind _lockrotation_scene (Variables|Default|GetLockRotation_Scene))
  (bind _relativerotation (Variables|/Script/Engine.SceneComponent|GetRelativeRotation _lockrotation_scene))
  (bind _returnvalue_2 (Math|Rotator|CombineRotators _relativerotation (Math|Rotator|MakeRotator _returnvalue 0.0 0.0)))
  ;[1 1 1] Forward lock rotation.
  (if (Variables|Default|GetIsLockRotating)
    (bind _output_get (Variables|Default|SetLockRotation (Math|Float|Clamp(Float) (.roll _returnvalue_2) -9e+01 0.0)))
    (Transformation|SetRelativeRotation (Variables|Default|GetLockRotation_Scene) (Math|Rotator|MakeRotator _output_get (.pitch _returnvalue_2) (.yaw _returnvalue_2)) false false)
    (CallFunction|LockpickForward)
    (if (== (Variables|Default|GetLockRotation) -9e+01)
      (Utilities|Time|PauseTimerbyHandle (Variables|Default|GetForwardLockTimer))
      (Default|CallOnLockpickCorrect))))

(event Custom|PlayLockJammed
  ;[1 1 1] Jammed lock rotation
  (bind _returnvalue (Utilities|Time|SetTimerbyEvent (delegate Custom|UpdateJammedLock) 0.05 true))
  (Variables|Default|SetJammedLock _returnvalue))

(event Custom|UpdateJammedLock
  ;[1 1 1] Jammed lock rotation
  (if (Variables|Default|GetIsLockRotating)
    (Utilities|FlowControl|Sequence
      (:then_0
        (Utilities|FlowControl|FlipFlop
          (:A
            (Variables|Default|SetJammedValue -3.0))
          (:B
            (Variables|Default|SetJammedValue 3.0))))
      (:then_1
        (bind _output_get (Variables|Default|SetLockRotation (Math|Float|Clamp(Float) (.roll (Math|Rotator|CombineRotators (Variables|/Script/Engine.SceneComponent|GetRelativeRotation (Variables|Default|GetLockRotation_Scene)) (Math|Rotator|MakeRotator (Variables|Default|GetJammedValue) 0.0 0.0))) -3.0 3.0)))
        (Transformation|SetRelativeRotation (Variables|Default|GetLockRotation_Scene) (Math|Rotator|MakeRotator _output_get (.pitch (Math|Rotator|CombineRotators (Variables|/Script/Engine.SceneComponent|GetRelativeRotation (Variables|Default|GetLockRotation_Scene)) (Math|Rotator|MakeRotator (Variables|Default|GetJammedValue) 0.0 0.0))) (.yaw (Math|Rotator|CombineRotators (Variables|/Script/Engine.SceneComponent|GetRelativeRotation (Variables|Default|GetLockRotation_Scene)) (Math|Rotator|MakeRotator (Variables|Default|GetJammedValue) 0.0 0.0)))) false false)
        (CallFunction|DrainLockpickHealth)))))

(event Custom|DrainLockpickHealth
  ;[1 1 1] Drain lockpick health.
  (bind _output_get (Variables|Default|SetLockpickHealth (Math|Float|Clamp(Float) (- (Variables|Default|GetLockpickHealth) 4.0) 0.0 1e+02)))
  (if (<= _output_get 0.0)
    (Utilities|FlowControl|DoOnce false
      (:Completed
        (Default|CallOnLockpickBroken)
        (CallFunction|LockpickAnim)
        (CallFunction|NewLockpick)))))

(event Custom|ResetLockpick
  ;[1 1 1] Drain lockpick health.
  (Utilities|FlowControl|DoOnce false) ; enters at Reset
)

(event Custom|LockpickingFailed
  (bind _returnvalue (Game|GetPlayerController 0))
  ;[1 1 1] Lockpicking failed.
  (Input|DisableInput _returnvalue)
  (Input|EnableInput (CallFunction|GetPlayer) _returnvalue)
  (bind _wb_lockpicking (Variables|Default|GetWB_Lockpicking)
    (:then
      (Widget|RemovefromParent _wb_lockpicking)
      (Variables|Default|SetWB_Lockpicking 0)
      (Actor|DestroyActor))
    (:else)))

(event Input|EnhancedActionEvents|EnhancedInputActionIA_Look
  (params (ActionValue :type Vector%202D%20Structure) (ElapsedSeconds :type Float%20%28double-precision%29) (TriggeredSeconds :type Float%20%28double-precision%29) (InputAction :type Input%20Action%20Object%20Reference :default "/Game/FirstPerson/Input/Actions/IA_Look.IA_Look"))
  (bind _returnvalue (* (.x ActionValue) -4.0))
  (bind _lockpickrotation_scene (Variables|Default|GetLockpickRotation_Scene))
  (bind _relativerotation (Variables|/Script/Engine.SceneComponent|GetRelativeRotation _lockpickrotation_scene))
  (bind _returnvalue_2 (Math|Rotator|CombineRotators _relativerotation (Math|Rotator|MakeRotator _returnvalue 0.0 0.0)))
  ;[1 1 1] Rotate Lockpick
  (if (not (Variables|Default|GetIsLockRotating))
    (bind _output_get (Variables|Default|SetLockpickRotation (Math|Float|Clamp(Float) (.roll _returnvalue_2) -9e+01 9e+01)))
    (Transformation|SetRelativeRotation (Variables|Default|GetLockpickRotation_Scene) (Math|Rotator|MakeRotator _output_get (.pitch _returnvalue_2) (.yaw _returnvalue_2)) false false)))

(event Input|EnhancedActionEvents|EnhancedInputActionIA_Lockpicking
  (params (ActionValue :type Boolean) (ElapsedSeconds :type Float%20%28double-precision%29) (TriggeredSeconds :type Float%20%28double-precision%29) (InputAction :type Input%20Action%20Object%20Reference :default "/Game/FirstPerson/Input/Actions/IA_Lockpicking.IA_Lockpicking"))
  ;[1 1 1] WASD input for lock rotation.
  (:Started
    (Variables|Default|SetIsLockRotating true)
    (if (CallFunction|CheckUnlockStatus)
      (CallFunction|ForwardLockRotation)
      (else
        (CallFunction|PlayLockJammed))))
  (:Completed
    (Variables|Default|SetIsLockRotating false)
    (if (not (Variables|Default|GetLockComplete))
      (CallFunction|BackwardLockRotation))))

(event Input|EnhancedActionEvents|EnhancedInputActionIA_Interaction
  (params (ActionValue :type Boolean) (ElapsedSeconds :type Float%20%28double-precision%29) (TriggeredSeconds :type Float%20%28double-precision%29) (InputAction :type Input%20Action%20Object%20Reference :default "/Game/FirstPerson/Input/Actions/IA_Interaction.IA_Interaction"))
  ;[1 1 1] Interaction Input
  (:Started
    (CallFunction|LockpickingFailed)))

(event EventBeginPlay
  ;[1 1 1] BeginPlay
  (CallFunction|GenerateLock)
  (EventDispatchers|BindEventtoOnLockpickCorrect (EventDispatchers|CreateEvent :!event Custom|LockpickingSuccessful)))

(fn ConstructionScript)

(fn LockpickForward
  (bind _lockpickrotation_scene (Variables|Default|GetLockpickRotation_Scene))
  (bind _relativelocation (Variables|/Script/Engine.SceneComponent|GetRelativeLocation _lockpickrotation_scene))
  (Transformation|SetRelativeLocation (Variables|Default|GetLockpickRotation_Scene) (Math|Vector|MakeVector (.x _relativelocation) (Math|Float|Clamp(Float) (- (.y _relativelocation) 0.16) -4.8 0.0) (Math|Float|Clamp(Float) (- (.z _relativelocation) 0.1) 2.0 5.0)) false false))

(fn LockpickBackward
  (bind _lockpickrotation_scene (Variables|Default|GetLockpickRotation_Scene))
  (bind _relativelocation (Variables|/Script/Engine.SceneComponent|GetRelativeLocation _lockpickrotation_scene))
  (Transformation|SetRelativeLocation (Variables|Default|GetLockpickRotation_Scene) (Math|Vector|MakeVector (.x _relativelocation) (Math|Float|Clamp(Float) (+ (.y _relativelocation) 0.32) -4.8 0.0) (Math|Float|Clamp(Float) (+ (.z _relativelocation) 0.2) 2.0 5.0)) false false))

(fn GenerateLock
  (Variables|Default|SetUnlockValue (Math|Random|RandomFloatinRange -9e+01 9e+01)))

(fn CheckUnlockStatus
  (return (Math|Float|NearlyEqual(Float) (Variables|Default|GetLockpickRotation) (Variables|Default|GetUnlockValue) (Variables|Default|GetErrorMargin))))