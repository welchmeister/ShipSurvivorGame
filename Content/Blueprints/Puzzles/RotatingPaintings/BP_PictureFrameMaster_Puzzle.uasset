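; Rotating painting puzzle piece that turns a quarter step per interaction and counts as completed at its answer position.
; Interaction sets completion from the next position before calling the timeline rotation, which ignores calls while moving and advances a four-step counter when finished.
; Each frame gathers all frames on BeginPlay and polls them on a looping timer.
; When all are completed, it stops polling, fires the puzzle-completed dispatcher and locks its interaction.
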(event Custom|RotatePainting
  ;[1 1 1] RotatingPainting
  (if (not (Variables|Default|GetFrameMoving?))
    (Variables|Default|SetFrameMoving? true)
    (Audio|PlaySoundatLocation "/Game/Meshes/PuzzleMeshes/Audio/DoorsAndFurnitures/PaintingRotation.PaintingRotation" (Variables|/Script/Engine.SceneComponent|GetRelativeLocation (Variables|Default|GetFrame)) "0, 0, 0" 1.0 1.0 0.0 0 0 0 0)
    (bind _rotation (Timeline|PaintingRotating PlayFromStart)
      (:Update
        (Transformation|SetRelativeRotation (Variables|Default|GetFrame) (Math|Rotator|MakeRotator 0.0 (Math|Float|Lerp (.pitch (Variables|Default|GetStartingRotationFrame)) (- (.pitch (Variables|Default|GetStartingRotationFrame)) 9e+01) _rotation) 0.0) false false))
      (:Finished
        (Variables|Default|SetStartingRotationFrame (Math|Rotator|MakeRotator 0.0 (Math|Float|Lerp (.pitch (Variables|Default|GetStartingRotationFrame)) (- (.pitch (Variables|Default|GetStartingRotationFrame)) 9e+01) _rotation) 0.0))
        (Variables|Default|SetFrameMoving? false)
        (bind _result (Math|Integer|IncrementInt (Variables|Default|GetFramePosition))
          (:%20%20
            (bind _output_get (Variables|Default|SetFramePosition _result))
            (if (> _output_get 3)
              (Variables|Default|SetFramePosition 0))))))))

(event Custom|PuzzleCheck
  ;[1 1 1] BeginPlay
  (Variables|Default|SetIsPuzzleSolved? true)
  (for _array_element (Variables|Default|GetAllPictureFrames)
    (if (not (Variables|BP_PictureFrameMaster_Puzzle_C|GetIsCompleted? _array_element))
      (Variables|Default|SetIsPuzzleSolved? false)))
  (if (Variables|Default|GetIsPuzzleSolved?)
    (Utilities|Time|ClearandInvalidateTimerbyHandle (Variables|Default|GetIsPuzzleComplete_TimerHandle))
    (Default|CallOnPuzzleCompleted)
    (Variables|Default|SetIsPuzzleCompleted? true)))

(event EventInteraction
  (params (Character :type First%20Person%20Character%20Object%20Reference) (HitActor :type Primitive%20Component%20Object%20Reference))
  ;[1 1 1] Interaction
  (if (not (Variables|Default|GetIsPuzzleCompleted?))
    (if (== (+ (Variables|Default|GetFramePosition) 1) (Variables|Default|GetPuzzleAnswer))
      (Variables|Default|SetIsCompleted? true)
      (CallFunction|RotatePainting)
      (else
        (Variables|Default|SetIsCompleted? false)
        (CallFunction|RotatePainting)))))

(event EventBeginPlay
  ;[1 1 1] BeginPlay
  (Variables|Default|SetStartingRotationFrame (Variables|/Script/Engine.SceneComponent|GetRelativeRotation (Variables|Default|GetFrame)))
  (bind _outactors (Actor|GetAllActorsOfClass "BP_PictureFrameMaster_Puzzle_C"))
  (Variables|Default|SetAllPictureFrames _outactors)
  (bind _returnvalue (Utilities|Time|SetTimerbyEvent (delegate Custom|PuzzleCheck) 0.25 true))
  (Variables|Default|SetIsPuzzleComplete_TimerHandle _returnvalue))

(fn ConstructionScript
  (|CallParentFunction))