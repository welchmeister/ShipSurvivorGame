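; Lockable puzzle door that swings open away from or toward the player's side using a dot product, with timeline-driven handle and sounds.
; Interaction toggles an unlocked door; a locked one compares DoorKeyID to the last player key, then animates the key and unlocks, or shakes.
; Box overlap shows instruction widgets while locked.
; An optional looping timer closes the door once the player exceeds CloseDistance.
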(event OnComponentBeginOverlap(Box)
  (params (OverlappedComponent :type Primitive%20Component%20Object%20Reference) (OtherActor :type Actor%20Object%20Reference) (OtherComp :type Primitive%20Component%20Object%20Reference) (OtherBodyIndex :type Integer) (bFromSweep :type Boolean) (SweepResult :type Hit%20Result%20Structure%20%28by%20ref%29))
  ;[1 1 1] Box Overlap Events
  (if (Variables|Default|GetLocked?)
    (Utilities|Casting|CastToFirstPersonCharacter OtherActor)
    (Rendering|SetVisibility (Variables|Default|GetWidget) true false)
    (Rendering|SetVisibility (Variables|Default|GetInstructionsWidget) true false)))

(event OnComponentEndOverlap(Box)
  (params (OverlappedComponent :type Primitive%20Component%20Object%20Reference) (OtherActor :type Actor%20Object%20Reference) (OtherComp :type Primitive%20Component%20Object%20Reference) (OtherBodyIndex :type Integer))
  ;[1 1 1] Box Overlap Events
  (if (Variables|Default|GetLocked?)
    (Utilities|Casting|CastToFirstPersonCharacter OtherActor)
    (Rendering|SetVisibility (Variables|Default|GetWidget) false false)
    (Rendering|SetVisibility (Variables|Default|GetInstructionsWidget) false false)))

(event Custom|OpenCloseDoor
  (bind _self self)
  ;[1 1 1] Open Close Logic
  (CallFunction|Sounds)
  (if (Variables|Default|GetDoorClosed?)
    (Variables|Default|SetDoorClosed? false)
    (CallFunction|RotateDoorHandle)
    (Variables|Default|SetDotProduct (Math|Vector|DotProduct (Math|Vector|Normalize (- (Transformation|GetActorLocation _self) (Transformation|GetActorLocation (Variables|Default|GetFirst%20Person%20Character)))) (Transformation|GetActorRightVector _self)))
    (bind _alpha (Timeline|Door_TL Play)
      (:Update
        (Transformation|SetRelativeRotation (Variables|Default|GetDoor) (Math|Rotator|MakeRotator 0.0 0.0 (Math|Float|Lerp 0.0 (Math|Float|SelectFloat 9e+01 -9e+01 (>= (Variables|Default|GetDotProduct) 0.0)) _alpha)) false false)))
    (else
      (Variables|Default|SetDoorClosed? true)
      (Timeline|Door_TL Reverse))))

(event Custom|AutoClose
  ;[1 1 1] Auto Close Door
  (if (Variables|Default|GetAutoClose?)
    (Utilities|Time|SetTimerbyEvent (delegate Custom|DoorAutoClose) 2.0 true)))

(event Custom|DoorAutoClose
  ;[1 1 1] Auto Close Door
  (if (not (Variables|Default|GetDoorClosed?))
    (if (> (Math|Vector|Distance(Vector) (Transformation|GetActorLocation (Variables|Default|GetFirst%20Person%20Character)) (Transformation|GetActorLocation)) (Variables|Default|GetCloseDistance))
      (CallFunction|OpenCloseDoor))))

(event Custom|CheckForKey
  ;[1 1 1] Check For Key
  (for _array_element (Variables|/Game/FirstPerson/FPSword/Blueprints/FirstPersonCharacter.FirstPersonCharacter_C|GetKeys (Variables|Default|GetFirst%20Person%20Character))
    _)
  (if (Utilities|Enum|Equal(Enum) _array_element (Variables|Default|GetDoorKeyID))
    (CallFunction|KeyAnimations)
    (Utilities|FlowControl|Delay 1.0)
    (CallFunction|UnlockDoor)
    (Variables|/Game/FirstPerson/FPSword/Blueprints/FirstPersonCharacter.FirstPersonCharacter_C|SetHasKey? (Variables|Default|GetFirst%20Person%20Character) false)
    (else
      (CallFunction|ShakeDoor))))

(event Custom|RotateDoorHandle
  ;[1 1 1] Rotate Door Handle
  (bind _alpha (Timeline|DoorHandle_TL PlayFromStart)
    (:Update
      (Transformation|SetRelativeRotation (Variables|Default|GetDoorHandle) (Math|Rotator|MakeRotator _alpha 0.0 0.0) false false))))

(event Custom|UnlockDoor
  (bind _unlocksound (Variables|Default|GetUnlockSound))
  ;[1 1 1] Unlock Door
  (Variables|Default|SetLocked? false)
  (Audio|PlaySoundatLocation _unlocksound (Transformation|GetWorldLocation (Variables|Default|GetDoor)) "0, 0, 0" 1.0 1.0 0.0 0 0 0 0)
  (Utilities|FlowControl|Delay (Variables|/Script/Engine.SoundBase|GetDuration _unlocksound))
  (CallFunction|OpenCloseDoor))

(event Custom|ShakeDoor
  ;[1 1 1] Door Shake
  (CallFunction|RotateDoorHandle)
  (Audio|PlaySoundatLocation "/Game/Meshes/PuzzleMeshes/Audio/DoorsAndFurnitures/Lock02.Lock02" (Transformation|GetActorLocation) "0, 0, 0" 1.0 1.0 0.0 0 0 0 0)
  (Utilities|FlowControl|FlipFlop
    (:A
      (bind _alpha (Timeline|ShakeDoor_TL PlayFromStart)
        (:Update
          (Transformation|SetRelativeRotation (Variables|Default|GetDoor) (Math|Rotator|MakeRotator 0.0 0.0 _alpha) false false))))
    (:B
      (Timeline|ShakeDoor_TL ReverseFromEnd))))

(event Custom|KeyAnimations
  (bind _keylocation (Variables|Default|GetKeyLocation))
  (Rendering|SetVisibility (Variables|Default|GetKey) true false)
  (bind _alpha (Timeline|KeyAnim_01 PlayFromStart)
    (:Update
      (Transformation|SetRelativeLocation (Variables|Default|GetKey) (Math|Vector|MakeVector (Math|Float|Lerp (.x _keylocation) (+ (.x _keylocation) 5.0) _alpha) (.y _keylocation) (.z _keylocation)) false false))
    (:Finished
      (bind _alpha_2 (Timeline|KeyAnim_02 PlayFromStart)
        (:Update
          (Transformation|SetRelativeRotation (Variables|Default|GetKey) (Math|Rotator|MakeRotator _alpha_2 0.0 0.0) false false))
        (:Finished
          (Rendering|SetVisibility (Variables|Default|GetKey) false false))))))

(event EventBeginPlay
  ;[1 1 1] Beginplay Event
  (bind _asfirst_person_character (Utilities|Casting|CastToFirstPersonCharacter (Game|GetPlayerCharacter 0)))
  (Variables|Default|SetFirst%20Person%20Character _asfirst_person_character)
  (Variables|Default|SetKeyLocation (Variables|/Script/Engine.SceneComponent|GetRelativeLocation (Variables|Default|GetKey)))
  (CallFunction|AutoClose))

(event EventInteraction
  (params (Character :type First%20Person%20Character%20Object%20Reference) (HitActor :type Primitive%20Component%20Object%20Reference))
  ;[1 1 1] Interaction Event
  (if (Variables|Default|GetLocked?)
    (CallFunction|CheckforKey)
    (else
      (CallFunction|OpenCloseDoor))))

(fn ConstructionScript)

(fn Sounds
  (bind _door (Variables|Default|GetDoor))
  (bind _returnvalue (Transformation|GetWorldLocation _door))
  (if (Variables|Default|GetLocked?)
    (Audio|PlaySoundatLocation (Variables|Default|GetLockedSound) _returnvalue "0, 0, 0" 1.0 1.0 0.0 0 0 0 0)
    (elif (Variables|Default|GetDoorClosed?)
      (Audio|PlaySoundatLocation (Variables|Default|GetOpenSound) _returnvalue "0, 0, 0" 1.0 1.0 0.0 0 0 0 0)
      (else
        (Audio|PlaySoundatLocation (Variables|Default|GetCloseSound) _returnvalue "0, 0, 0" 1.0 1.0 0.0 0 0 0 0)))))