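; Interactive puzzle door that, while locked and unsolved, opens a jigsaw widget once on interaction and freezes player movement and look.
; Otherwise interaction toggles a timeline swing, using a dot product to open away from or toward the player's side.
; A looping timer can auto-close it beyond a set distance.
; Unlock and shake events drive sounds and handle animation, while box overlaps show prompt widgets when locked.
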(event OnComponentBeginOverlap(Box)
  (params (OverlappedComponent :type Primitive%20Component%20Object%20Reference) (OtherActor :type Actor%20Object%20Reference) (OtherComp :type Primitive%20Component%20Object%20Reference) (OtherBodyIndex :type Integer) (bFromSweep :type Boolean) (SweepResult :type Hit%20Result%20Structure%20%28by%20ref%29))
  ;[1 1 1] Box Overlap Events to display widget instructions for door.
  (if (Variables|Default|GetLocked?)
    (Utilities|Casting|CastToFirstPersonCharacter OtherActor)
    (Rendering|SetVisibility (Variables|Default|GetInteractWidget) true false)
    (Rendering|SetVisibility (Variables|Default|GetInstructionsWidget) true false)
    (else
      (Rendering|SetVisibility (Variables|Default|GetInteractWidget) false false)
      (Rendering|SetVisibility (Variables|Default|GetInstructionsWidget) false false))))

(event OnComponentEndOverlap(Box)
  (params (OverlappedComponent :type Primitive%20Component%20Object%20Reference) (OtherActor :type Actor%20Object%20Reference) (OtherComp :type Primitive%20Component%20Object%20Reference) (OtherBodyIndex :type Integer))
  ;[1 1 1] Box Overlap Events to display widget instructions for door.
  (if (Variables|Default|GetLocked?)
    (Utilities|Casting|CastToFirstPersonCharacter OtherActor)
    (Rendering|SetVisibility (Variables|Default|GetInteractWidget) false false)
    (Rendering|SetVisibility (Variables|Default|GetInstructionsWidget) false false)))

(event Custom|OpenCloseDoor
  (bind _self self)
  ;[1 1 1] Open Close Logic
  (Utilities|FlowControl|DoOnce false
    (:Completed
      (CallFunction|Sounds)
      (if (Variables|Default|GetDoorClosed?)
        (Variables|Default|SetDoorClosed? false)
        (CallFunction|RotateDoorHandle)
        (Variables|Default|SetDotProduct (Math|Vector|DotProduct (Math|Vector|Normalize (- (Transformation|GetActorLocation _self) (Transformation|GetActorLocation (Variables|Default|GetFirst%20Person%20Character)))) (Transformation|GetActorRightVector _self)))
        (bind _alpha (Timeline|Door_TL Play)
          (:Update
            (Transformation|SetRelativeRotation (Variables|Default|GetDoor) (Math|Rotator|MakeRotator 0.0 0.0 (Math|Float|Lerp 0.0 (Math|Float|SelectFloat 9e+01 -9e+01 (>= (Variables|Default|GetDotProduct) 0.0)) _alpha)) false false))
          (:Finished
            (CallFunction|ResetOpeningDoor)))
        (else
          (Variables|Default|SetDoorClosed? true)
          (Timeline|Door_TL Reverse))))))

(event Custom|AutoClose
  ;[1 1 1] Auto Close Door
  (if (Variables|Default|GetAutoClose?)
    (Utilities|Time|SetTimerbyEvent (delegate Custom|DoorAutoClose) 2.0 true)))

(event Custom|DoorAutoClose
  ;[1 1 1] Auto Close Door
  (if (not (Variables|Default|GetDoorClosed?))
    (if (> (Math|Vector|Distance(Vector) (Transformation|GetActorLocation (Variables|Default|GetFirst%20Person%20Character)) (Transformation|GetActorLocation)) (Variables|Default|GetCloseDistance))
      (CallFunction|OpenCloseDoor))))

(event Custom|Reset%20Opening%20Door
  (bind _self self)
  ;[1 1 1] Open Close Logic
  (Utilities|FlowControl|DoOnce false) ; enters at Reset
)

(event Custom|RotateDoorHandle
  ;[1 1 1] Rotate Door Handle
  (bind _alpha (Timeline|DoorHandle_TL PlayFromStart)
    (:Update
      (Transformation|SetRelativeRotation (Variables|Default|GetDoorHandle) (Math|Rotator|MakeRotator _alpha 0.0 0.0) false false))))

(event Custom|UnlockDoor
  (bind _unlocksound (Variables|Default|GetUnlockSound))
  ;[1 1 1] Unlock Door
  (Variables|Default|SetLocked? false)
  (Audio|PlaySoundatLocation _unlocksound (Transformation|GetWorldLocation (Variables|Default|GetDoor)) "0, 0, 0" 1.0 1.0 0.0 0 0 0 0)
  (Utilities|FlowControl|Delay (Variables|/Script/Engine.SoundBase|GetDuration _unlocksound))
  (CallFunction|OpenCloseDoor)
  (Rendering|SetVisibility (Variables|Default|GetInteractWidget) false false)
  (Rendering|SetVisibility (Variables|Default|GetInstructionsWidget) false false))

(event Custom|ShakeDoor
  ;[1 1 1] Door Shake
  (CallFunction|RotateDoorHandle)
  (Audio|PlaySoundatLocation "/Game/Meshes/PuzzleMeshes/Audio/DoorsAndFurnitures/Lock02.Lock02" (Transformation|GetActorLocation) "0, 0, 0" 1.0 1.0 0.0 0 0 0 0)
  (Utilities|FlowControl|FlipFlop
    (:A
      (bind _alpha (Timeline|ShakeDoor_TL PlayFromStart)
        (:Update
          (Transformation|SetRelativeRotation (Variables|Default|GetDoor) (Math|Rotator|MakeRotator 0.0 0.0 _alpha) false false))))
    (:B
      (Timeline|ShakeDoor_TL ReverseFromEnd))))

(event Custom|DoorUnlock
  ;[1 1 1] Unlock Door
  (Variables|Default|SetLocked? false)
  (CallFunction|Sounds)
  (CallFunction|RotateDoorHandle))

(event EventInteraction
  (params (Character :type First%20Person%20Character%20Object%20Reference) (HitActor :type Primitive%20Component%20Object%20Reference))
  (bind _returnvalue (Game|GetPlayerController 0))
  ;[1 1 1] Interaction Event
  (if (not (Variables|Default|GetPuzzleCompleted))
    (if (Variables|Default|GetLocked?)
      (Utilities|FlowControl|DoOnce false
        (:Completed
          (bind _returnvalue_2 (UserInterface|CreateWidget "/Game/Blueprints/Puzzles/Jigsaw/JigsawWidget.JigsawWidget_C"))
          (UserInterface|Viewport|AddtoViewport _returnvalue_2 0)
          (Variables|/Script/Engine.PlayerController|SetbShowMouseCursor _returnvalue true)
          (Pawn|Components|CharacterMovement|DisableMovement (Variables|/Script/Engine.Character|GetCharacterMovement (Game|GetPlayerCharacter 0)))
          (Input|SetIgnoreLookInput _returnvalue true)))
      (else
        (CallFunction|OpenCloseDoor)))
    (else
      (CallFunction|OpenCloseDoor))))

(event EventBeginPlay
  ;[1 1 1] Beginplay Event
  (bind _asfirst_person_character (Utilities|Casting|CastToFirstPersonCharacter (Game|GetPlayerCharacter 0)))
  (Variables|Default|SetFirst%20Person%20Character _asfirst_person_character)
  (CallFunction|AutoClose))

(fn ConstructionScript)

(fn Sounds
  (bind _door (Variables|Default|GetDoor))
  (bind _returnvalue (Transformation|GetWorldLocation _door))
  (if (Variables|Default|GetLocked?)
    (Audio|PlaySoundatLocation (Variables|Default|GetLockedSound) _returnvalue "0, 0, 0" 1.0 1.0 0.0 0 0 0 0)
    (elif (Variables|Default|GetDoorClosed?)
      (Audio|PlaySoundatLocation (Variables|Default|GetOpenSound) _returnvalue "0, 0, 0" 1.0 1.0 0.0 0 0 0 0)
      (else
        (Audio|PlaySoundatLocation (Variables|Default|GetCloseSound) _returnvalue "0, 0, 0" 1.0 1.0 0.0 0 0 0 0)))))