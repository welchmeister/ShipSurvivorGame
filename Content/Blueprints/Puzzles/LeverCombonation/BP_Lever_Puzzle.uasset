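; Lever combination puzzle where the player flips four levers into a fixed on/off pattern.
; Interacting with the panel blends the view to the puzzle, enables cursor clicks and freezes movement until Back or completion restores control.
; Mouse clicks or gamepad events toggle each lever through a FlipFlop and rotation timeline, which triggers the answer check on finishing.
; Solving fires OnPuzzleCompleted and locks the puzzle; box overlaps control prompt widgets.
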(event OnClicked(Lever3)
  (params (TouchedComponent :type Primitive%20Component%20Object%20Reference) (ButtonPressed :type Key%20Structure :default "None"))
  ;[1 1 1] On Clicked Event (Levers)
  (Audio|PlaySound2D "/Game/Meshes/PuzzleMeshes/Audio/DoorsAndFurnitures/HandleOpen01.HandleOpen01" 1.0 1.0 0.0 0 0)
  (Utilities|FlowControl|FlipFlop
    (:A
      (Variables|Default|SetLever03_On true)
      (bind _alpha (Timeline|RotateLever03 Play)
        (:Update
          (Transformation|SetRelativeRotation (Variables|Default|GetLever3) (Math|Rotator|MakeRotator _alpha 0.0 0.0) false false))
        (:Finished
          (CallFunction|AnswerCheck))))
    (:B
      (Variables|Default|SetLever03_On false)
      (Timeline|RotateLever03 Reverse))))

(event OnClicked(Lever4)
  (params (TouchedComponent :type Primitive%20Component%20Object%20Reference) (ButtonPressed :type Key%20Structure :default "None"))
  ;[1 1 1] On Clicked Event (Levers)
  (Audio|PlaySound2D "/Game/Meshes/PuzzleMeshes/Audio/DoorsAndFurnitures/HandleOpen01.HandleOpen01" 1.0 1.0 0.0 0 0)
  (Utilities|FlowControl|FlipFlop
    (:A
      (Variables|Default|SetLever04_On true)
      (bind _alpha (Timeline|RotateLever04 Play)
        (:Update
          (Transformation|SetRelativeRotation (Variables|Default|GetLever4) (Math|Rotator|MakeRotator _alpha 0.0 0.0) false false))
        (:Finished
          (CallFunction|AnswerCheck))))
    (:B
      (Variables|Default|SetLever04_On false)
      (Timeline|RotateLever04 Reverse))))

(event OnComponentBeginOverlap(Box)
  (params (OverlappedComponent :type Primitive%20Component%20Object%20Reference) (OtherActor :type Actor%20Object%20Reference) (OtherComp :type Primitive%20Component%20Object%20Reference) (OtherBodyIndex :type Integer) (bFromSweep :type Boolean) (SweepResult :type Hit%20Result%20Structure%20%28by%20ref%29))
  ;[1 1 1] Box Overlap Events
  (if (or (Variables|Default|GetIsPuzzleCompleted?) (Variables|Default|GetIsPuzzleActivated?))
    (Rendering|SetVisibility (Variables|Default|GetInteractWidget) false false)
    (Rendering|SetVisibility (Variables|Default|GetInstructionsWidget) false false)
    (else
      (Utilities|Casting|CastToFirstPersonCharacter OtherActor)
      (Rendering|SetVisibility (Variables|Default|GetInteractWidget) true false)
      (Rendering|SetVisibility (Variables|Default|GetInstructionsWidget) true false))))

(event OnComponentEndOverlap(Box)
  (params (OverlappedComponent :type Primitive%20Component%20Object%20Reference) (OtherActor :type Actor%20Object%20Reference) (OtherComp :type Primitive%20Component%20Object%20Reference) (OtherBodyIndex :type Integer))
  ;[1 1 1] Box Overlap Events
  (if (not (or (Variables|Default|GetIsPuzzleCompleted?) (Variables|Default|GetIsPuzzleActivated?)))
    (Utilities|Casting|CastToFirstPersonCharacter OtherActor)
    (Rendering|SetVisibility (Variables|Default|GetInteractWidget) false false)
    (Rendering|SetVisibility (Variables|Default|GetInstructionsWidget) false false)))

(event OnClicked(Lever1)
  (params (TouchedComponent :type Primitive%20Component%20Object%20Reference) (ButtonPressed :type Key%20Structure :default "None"))
  ;[1 1 1] On Clicked Event (Levers)
  (Audio|PlaySound2D "/Game/Meshes/PuzzleMeshes/Audio/DoorsAndFurnitures/HandleOpen01.HandleOpen01" 1.0 1.0 0.0 0 0)
  (Utilities|FlowControl|FlipFlop
    (:A
      (Variables|Default|SetLever01_On true)
      (bind _alpha (Timeline|RotateLever01 Play)
        (:Update
          (Transformation|SetRelativeRotation (Variables|Default|GetLever1) (Math|Rotator|MakeRotator _alpha 0.0 0.0) false false))
        (:Finished
          (CallFunction|AnswerCheck))))
    (:B
      (Variables|Default|SetLever01_On false)
      (Timeline|RotateLever01 Reverse))))

(event OnClicked(Lever2)
  (params (TouchedComponent :type Primitive%20Component%20Object%20Reference) (ButtonPressed :type Key%20Structure :default "None"))
  ;[1 1 1] On Clicked Event (Levers)
  (Audio|PlaySound2D "/Game/Meshes/PuzzleMeshes/Audio/DoorsAndFurnitures/HandleOpen01.HandleOpen01" 1.0 1.0 0.0 0 0)
  (Utilities|FlowControl|FlipFlop
    (:A
      (Variables|Default|SetLever02_On true)
      (bind _alpha (Timeline|RotateLever02 Play)
        (:Update
          (Transformation|SetRelativeRotation (Variables|Default|GetLever2) (Math|Rotator|MakeRotator _alpha 0.0 0.0) false false))
        (:Finished
          (CallFunction|AnswerCheck))))
    (:B
      (Variables|Default|SetLever02_On false)
      (Timeline|RotateLever02 Reverse))))

(event Custom|Answer%20Check
  ;[1 1 1] Check to see if levers are in correct sequence. Then open door and complete puzzle.
  (if (and (Variables|Default|GetLever02_On) (Variables|Default|GetLever04_On))
    (if (not (Variables|Default|GetLever01_On))
      (if (not (Variables|Default|GetLever03_On))
        (CallFunction|LeverPuzzleComplete)
        (Default|CallOnPuzzleCompleted)
        (Variables|Default|SetIsPuzzleCompleted? true)
        (Rendering|SetVisibility (Variables|Default|GetInteractWidget) false false)
        (Rendering|SetVisibility (Variables|Default|GetInstructionsWidget) false false)))))

(event Custom|Gamepad%20Click%20Lever%202
  ;[1 1 1] On Clicked Event (Levers)
  (Audio|PlaySound2D "/Game/Meshes/PuzzleMeshes/Audio/DoorsAndFurnitures/HandleOpen01.HandleOpen01" 1.0 1.0 0.0 0 0)
  (Utilities|FlowControl|FlipFlop
    (:A
      (Variables|Default|SetLever02_On true)
      (bind _alpha (Timeline|RotateLever02 Play)
        (:Update
          (Transformation|SetRelativeRotation (Variables|Default|GetLever2) (Math|Rotator|MakeRotator _alpha 0.0 0.0) false false))
        (:Finished
          (CallFunction|AnswerCheck))))
    (:B
      (Variables|Default|SetLever02_On false)
      (Timeline|RotateLever02 Reverse))))

(event Custom|LeverPuzzleComplete
  (bind _returnvalue (Game|GetPlayerController 0))
  (bind _returnvalue_2 (Game|GetPlayerController 0))
  ;[1 1 1] Interaction
  (Game|Player|SetViewTargetwithBlend (Game|GetPlayerController 0) (Variables|Default|GetPlayerRef) 0.5 "VTBlend_Linear" 0.0 false)
  (Variables|/Script/Engine.PlayerController|SetbEnableClickEvents _returnvalue false)
  (Variables|/Script/Engine.PlayerController|SetbShowMouseCursor _returnvalue false)
  (Pawn|Components|CharacterMovement|SetMovementMode (Variables|/Script/Engine.Character|GetCharacterMovement (Variables|Default|GetPlayerRef)) "MOVE_Walking" 0)
  (Input|ResetIgnoreLookInput _returnvalue_2)
  (Input|SetIgnoreLookInput _returnvalue_2 false)
  (Input|SetInputModeGameOnly _returnvalue_2 false)
  (Variables|Default|SetIsPuzzleActivated? false)
  (Rendering|SetVisibility (Variables|Default|GetInteractWidget) true false)
  (Rendering|SetVisibility (Variables|Default|GetInstructionsWidget) true false))

(event Custom|Gamepad%20Click%20Lever%201
  ;[1 1 1] On Clicked Event (Levers)
  (Audio|PlaySound2D "/Game/Meshes/PuzzleMeshes/Audio/DoorsAndFurnitures/HandleOpen01.HandleOpen01" 1.0 1.0 0.0 0 0)
  (Utilities|FlowControl|FlipFlop
    (:A
      (Variables|Default|SetLever01_On true)
      (bind _alpha (Timeline|RotateLever01 Play)
        (:Update
          (Transformation|SetRelativeRotation (Variables|Default|GetLever1) (Math|Rotator|MakeRotator _alpha 0.0 0.0) false false))
        (:Finished
          (CallFunction|AnswerCheck))))
    (:B
      (Variables|Default|SetLever01_On false)
      (Timeline|RotateLever01 Reverse))))

(event Custom|Gamepad%20Click%20Lever%204
  ;[1 1 1] On Clicked Event (Levers)
  (Audio|PlaySound2D "/Game/Meshes/PuzzleMeshes/Audio/DoorsAndFurnitures/HandleOpen01.HandleOpen01" 1.0 1.0 0.0 0 0)
  (Utilities|FlowControl|FlipFlop
    (:A
      (Variables|Default|SetLever04_On true)
      (bind _alpha (Timeline|RotateLever04 Play)
        (:Update
          (Transformation|SetRelativeRotation (Variables|Default|GetLever4) (Math|Rotator|MakeRotator _alpha 0.0 0.0) false false))
        (:Finished
          (CallFunction|AnswerCheck))))
    (:B
      (Variables|Default|SetLever04_On false)
      (Timeline|RotateLever04 Reverse))))

(event Custom|Gamepad%20Click%20Lever%203
  ;[1 1 1] On Clicked Event (Levers)
  (Audio|PlaySound2D "/Game/Meshes/PuzzleMeshes/Audio/DoorsAndFurnitures/HandleOpen01.HandleOpen01" 1.0 1.0 0.0 0 0)
  (Utilities|FlowControl|FlipFlop
    (:A
      (Variables|Default|SetLever03_On true)
      (bind _alpha (Timeline|RotateLever03 Play)
        (:Update
          (Transformation|SetRelativeRotation (Variables|Default|GetLever3) (Math|Rotator|MakeRotator _alpha 0.0 0.0) false false))
        (:Finished
          (CallFunction|AnswerCheck))))
    (:B
      (Variables|Default|SetLever03_On false)
      (Timeline|RotateLever03 Reverse))))

(event Input|EnhancedActionEvents|EnhancedInputActionIA_Action
  (params (ActionValue :type Boolean) (ElapsedSeconds :type Float%20%28double-precision%29) (TriggeredSeconds :type Float%20%28double-precision%29) (InputAction :type Input%20Action%20Object%20Reference :default "/Game/FirstPerson/Input/Actions/IA_Action.IA_Action"))
  (bind _widgetinteraction (Variables|Default|GetWidgetInteraction))
  ;[1 1 1] Send line trace to hit widget button
  (:Started
    (Class|WidgetInteractionComponent|PressPointerKey _widgetinteraction "LeftMouseButton"))
  (:Completed
    (Class|WidgetInteractionComponent|ReleasePointerKey _widgetinteraction "LeftMouseButton")))

(event Input|EnhancedActionEvents|EnhancedInputActionIA_Back
  (params (ActionValue :type Boolean) (ElapsedSeconds :type Float%20%28double-precision%29) (TriggeredSeconds :type Float%20%28double-precision%29) (InputAction :type Input%20Action%20Object%20Reference :default "/Game/FirstPerson/Input/Actions/IA_Back.IA_Back"))
  (bind _returnvalue (Game|GetPlayerController 0))
  (bind _returnvalue_2 (Game|GetPlayerController 0))
  ;[1 1 1] Interaction
  (:Started
    (if (Variables|Default|GetIsPuzzleActivated?)
      (Game|Player|SetViewTargetwithBlend (Game|GetPlayerController 0) (Variables|Default|GetPlayerRef) 0.5 "VTBlend_Linear" 0.0 false)
      (Variables|/Script/Engine.PlayerController|SetbEnableClickEvents _returnvalue false)
      (Variables|/Script/Engine.PlayerController|SetbShowMouseCursor _returnvalue false)
      (Pawn|Components|CharacterMovement|SetMovementMode (Variables|/Script/Engine.Character|GetCharacterMovement (Variables|Default|GetPlayerRef)) "MOVE_Walking" 0)
      (Input|ResetIgnoreLookInput _returnvalue_2)
      (Input|SetIgnoreLookInput _returnvalue_2 false)
      (Input|SetInputModeGameOnly _returnvalue_2 false)
      (Variables|Default|SetIsPuzzleActivated? false)
      (Rendering|SetVisibility (Variables|Default|GetInteractWidget) true false)
      (Rendering|SetVisibility (Variables|Default|GetInstructionsWidget) true false))))

(event EventBeginPlay
  ;[1 1 1] Beginplay
  (|CallParentFunction)
  (Input|EnableInput (Game|GetPlayerController 0)))

(event EventInteraction
  (params (Character :type First%20Person%20Character%20Object%20Reference) (HitActor :type Primitive%20Component%20Object%20Reference))
  (bind _returnvalue (Game|GetPlayerController 0))
  ;[1 1 1] Interaction
  (if (not (Variables|Default|GetIsPuzzleCompleted?))
    (if (Utilities|Enum|Equal(Enum) (Utilities|GetDisplayName HitActor) "BP_Lever_Puzzle.Panel Shape_Cube")
      (Game|Player|SetViewTargetwithBlend _returnvalue self 0.5 "VTBlend_Linear" 0.0 false)
      (Variables|/Script/Engine.PlayerController|SetbEnableClickEvents _returnvalue true)
      (Variables|/Script/Engine.PlayerController|SetbShowMouseCursor _returnvalue true)
      (Pawn|Components|CharacterMovement|DisableMovement (Variables|/Script/Engine.Character|GetCharacterMovement (Variables|Default|GetPlayerRef)))
      (Input|SetInputModeGameandUI _returnvalue 0 "LockAlways" true false)
      (Variables|Default|SetIsPuzzleActivated? true)
      (Rendering|SetVisibility (Variables|Default|GetInteractWidget) false false)
      (Rendering|SetVisibility (Variables|Default|GetInstructionsWidget) false false)
      (Default|Detach (Variables|/Game/FirstPerson/FPSword/Blueprints/FirstPersonCharacter.FirstPersonCharacter_C|GetAC_Inventory (Variables|Default|GetPlayerRef))))))

(fn ConstructionScript
  (|CallParentFunction))