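; Keypad light puzzle that takes over the player's view on interaction, showing the cursor and disabling movement and look until exit.
; Clicks trace from the mouse, toggling the hit button's state and material plus the linked buttons in ButtonConfig entry 0, whichever button is pressed.
; When all buttons are lit, it returns view and control to the player and calls OnPuzzleCompleted; Q also exits.
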(event Custom|ExitView
  (bind _returnvalue (Game|GetPlayerController 0))
  (bind _returnvalue_2 (Game|GetPlayerController 0))
  (bind _returnvalue_3 (Game|GetPlayerCharacter 0))
  ;[1 1 1] Exit View Event
  (Game|Player|SetViewTargetwithBlend _returnvalue_2 _returnvalue_3 0.5 "VTBlend_Linear" 0.0 false)
  (Input|DisableInput _returnvalue_2)
  (Pawn|Components|CharacterMovement|SetMovementMode (Variables|/Script/Engine.Character|GetCharacterMovement _returnvalue_3) "MOVE_Walking" 0)
  (Variables|/Script/Engine.PlayerController|SetbShowMouseCursor _returnvalue_2 false)
  (Input|ResetIgnoreLookInput _returnvalue)
  (Input|SetIgnoreLookInput _returnvalue false)
  (Input|SetInputModeGameOnly _returnvalue false))

(event Input|EnhancedActionEvents|EnhancedInputActionIA_Action
  (params (ActionValue :type Boolean) (ElapsedSeconds :type Float%20%28double-precision%29) (TriggeredSeconds :type Float%20%28double-precision%29) (InputAction :type Input%20Action%20Object%20Reference :default "/Game/FirstPerson/Input/Actions/IA_Action.IA_Action"))
  (bind _returnvalue (Game|GetPlayerController 0))
  (bind _buttonconfig (Variables|Default|GetButtonConfig))
  (bind (_worldlocation _worlddirection _returnvalue_2) (Game|Player|ConvertMouseLocationToWorldSpace _returnvalue))
  (bind (_value _returnvalue_3) (Utilities|Map|Find _buttonconfig 0))
  ;[1 1 1] Action Input - Sends line trace from mouse position to object behind it. Checks to see if swith and if yes then turn on. Then checks to see if all switched are lit up and then complete the puzzle.
  (:Started
    (Utilities|IsValid _returnvalue
      (:Is%20Valid
        (if _returnvalue_2
          (bind (_outhit _returnvalue_4) (Collision|LineTraceByChannel _worldlocation (+ (* _worlddirection 1.5e+02) _worldlocation) "TraceTypeQuery1" false 0 "None" false))
          (if _returnvalue_4
            (Audio|PlaySoundatLocation "/Game/Meshes/PuzzleMeshes/Audio/Button/ButtonOn04.ButtonOn04" (.ImpactPoint (Collision|BreakHitResult _outhit)) "0, 0, 0" 1.0 1.0 0.0 0 0 0 0)
            (bind _asstatic_mesh_component (Utilities|Casting|CastToStaticMeshComponent (.HitComponent (Collision|BreakHitResult _outhit))))
            (CallFunction|ToggleActivation (Utilities|Array|FindItem (Variables|Default|GetButtons) _asstatic_mesh_component))
            (if _returnvalue_3
              (for _array_element (Utilities|Struct|BreakST_ButtonsToActivate _value)
                (CallFunction|ToggleActivation _array_element)))
            (bind _succees_ (CallFunction|CheckAnswer))
            (if _succees_
              (Utilities|FlowControl|Delay 0.5)
              (CallFunction|ExitView)
              (Default|CallOnPuzzleCompleted))))))))

(event EventInteraction
  (params (Character :type First%20Person%20Character%20Object%20Reference) (HitActor :type Primitive%20Component%20Object%20Reference))
  (bind _returnvalue (Game|GetPlayerController 0))
  (bind _asfirst_person_character (CallFunction|GetPlayer))
  ;[1 1 1] Interaction Event
  (Game|Player|SetViewTargetwithBlend (Game|GetPlayerController 0) self 0.5 "VTBlend_Linear" 0.0 false)
  (Pawn|Components|CharacterMovement|DisableMovement (Variables|/Script/Engine.Character|GetCharacterMovement (Game|GetPlayerCharacter 0)))
  (Input|SetIgnoreLookInput _returnvalue true)
  (Utilities|FlowControl|Delay 0.5)
  (Input|EnableInput _returnvalue)
  (Variables|/Script/Engine.PlayerController|SetbShowMouseCursor _returnvalue true)
  (Input|SetInputModeGameandUI _returnvalue 0 "LockAlways" true false)
  (Default|Detach (Variables|/Game/FirstPerson/FPSword/Blueprints/FirstPersonCharacter.FirstPersonCharacter_C|GetAC_Inventory _asfirst_person_character))
  (Variables|/Game/FirstPerson/FPSword/Blueprints/FirstPersonCharacter.FirstPersonCharacter_C|SetOverlayState _asfirst_person_character "NewEnumerator4"))

(event Input|KeyboardEvents|Q
  (params (Key :type Key%20Structure :default "None"))
  ;[1 1 1] Exit View Event
  (:Pressed
    (CallFunction|ExitView)))

(fn ConstructionScript
  (Variables|Default|SetButtons (Utilities|Array|MakeArray (Variables|Default|GetButton0) (Variables|Default|GetButton1) (Variables|Default|GetButton2) (Variables|Default|GetButton3) (Variables|Default|GetButton4) (Variables|Default|GetButton5) (Variables|Default|GetButton6) (Variables|Default|GetButton7) (Variables|Default|GetButton8) (Variables|Default|GetButton9))))

(fn ToggleActivation
  (params (ButtonIndex :type Integer))
  (bind _buttonactivationstate (Variables|Default|GetButtonActivationState))
  (bind _buttons (Variables|Default|GetButtons))
  (bind _output (Utilities|Array|Get(acopy) _buttons ButtonIndex))
  (Utilities|Array|SetArrayElem _buttonactivationstate ButtonIndex (not (Utilities|Array|Get(acopy) _buttonactivationstate ButtonIndex)))
  (if (Utilities|Array|Get(acopy) _buttonactivationstate ButtonIndex)
    (Rendering|Material|SetMaterial _output 0 "/Game/Meshes/PuzzleMeshes/Materials/M_ButtonOn.M_ButtonOn")
    (else
      (Utilities|IsValid _output
        (:Is%20Valid
          (Rendering|Material|SetMaterial _output 0 "/Game/Meshes/PuzzleMeshes/Materials/M_ButtonOff.M_ButtonOff"))))))

(fn CheckAnswer
  (if (== (Utilities|Array|Length (Variables|Default|GetButtons)) (Utilities|Array|Length (Variables|Default|GetButtonActivationState)))
    (for _array_element (Variables|Default|GetButtonActivationState)
      (if (not _array_element)
        (return false)))
    (return true)))