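; BP_Cannon is an interactable cannon that fires cannonballs from the interacting character's inventory, showing instruction and interact widgets while the player overlaps its box.
; Interaction requires an active "cannonball" item, then spawns a projectile, explosion effect and sound at SpawnPoint.
; It decrements the quantity by reassigning Items to a new single-entry map.
; At zero, Drop removes the item, unbinds its slot and clears the hand.
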(event OnComponentBeginOverlap(Box)
  (params (OverlappedComponent :type Primitive%20Component%20Object%20Reference) (OtherActor :type Actor%20Object%20Reference) (OtherComp :type Primitive%20Component%20Object%20Reference) (OtherBodyIndex :type Integer) (bFromSweep :type Boolean) (SweepResult :type Hit%20Result%20Structure%20%28by%20ref%29))
  ;[1 1 1] Box Overlap Events (Sets widgets on and off)
  (if (== OtherActor (CallFunction|GetPlayer))
    (Rendering|SetVisibility (Variables|Default|GetInstructionsWidget) true false)
    (Rendering|SetVisibility (Variables|Default|GetInteractWidget) true false)))

(event OnComponentEndOverlap(Box)
  (params (OverlappedComponent :type Primitive%20Component%20Object%20Reference) (OtherActor :type Actor%20Object%20Reference) (OtherComp :type Primitive%20Component%20Object%20Reference) (OtherBodyIndex :type Integer))
  ;[1 1 1] Box Overlap Events (Sets widgets on and off)
  (if (== OtherActor (CallFunction|GetPlayer))
    (Rendering|SetVisibility (Variables|Default|GetInstructionsWidget) false false)
    (Rendering|SetVisibility (Variables|Default|GetInteractWidget) false false)))

(event EventInteraction
  (params (Character :type First%20Person%20Character%20Object%20Reference) (HitActor :type Primitive%20Component%20Object%20Reference))
  (bind _ac_inventory (Variables|/Game/FirstPerson/FPSword/Blueprints/FirstPersonCharacter.FirstPersonCharacter_C|GetAC_Inventory Character))
  (bind _activeitem (Variables|/Game/Blueprints/Inventory/ActorComponents/AC_Inventory.AC_Inventory_C|GetActiveItem _ac_inventory))
  ;[1 1 1] Interaction
  (Variables|Default|SetAC%20Inventory _ac_inventory)
  (if (== _activeitem "cannonball")
    (bind _output_get (Variables|Default|SetCurrent _activeitem))
    (if (.Success (Default|GetItem (Variables|Default|GetAC%20Inventory) _output_get))
      (bind _result (Math|Integer|DecrementInt (.Quantity (Utilities|Struct|BreakST_Inventory_Item (.Value (Default|GetItem (Variables|Default|GetAC%20Inventory) _output_get)))))
        (:%20%20
          (Variables|/Game/Blueprints/Inventory/ActorComponents/AC_Inventory.AC_Inventory_C|SetItems (Variables|Default|GetAC%20Inventory) (Utilities|Map|MakeMap (Variables|Default|GetCurrent) (Utilities|Struct|MakeST_Inventory_Item (.ID (Utilities|Struct|BreakST_Inventory_Item (.Value (Default|GetItem (Variables|Default|GetAC%20Inventory) _output_get)))) (.Type (Utilities|Struct|BreakST_Inventory_Item (.Value (Default|GetItem (Variables|Default|GetAC%20Inventory) _output_get)))) (.DisplayName (Utilities|Struct|BreakST_Inventory_Item (.Value (Default|GetItem (Variables|Default|GetAC%20Inventory) _output_get)))) (.ShortDescription (Utilities|Struct|BreakST_Inventory_Item (.Value (Default|GetItem (Variables|Default|GetAC%20Inventory) _output_get)))) _result (.Thumbnail (Utilities|Struct|BreakST_Inventory_Item (.Value (Default|GetItem (Variables|Default|GetAC%20Inventory) _output_get)))) (.PickupMesh (Utilities|Struct|BreakST_Inventory_Item (.Value (Default|GetItem (Variables|Default|GetAC%20Inventory) _output_get)))) (.PickupMeshStatic (Utilities|Struct|BreakST_Inventory_Item (.Value (Default|GetItem (Variables|Default|GetAC%20Inventory) _output_get)))) (.HoldableSettings (Utilities|Struct|BreakST_Inventory_Item (.Value (Default|GetItem (Variables|Default|GetAC%20Inventory) _output_get)))))))
          (Game|SpawnActorfromClass "/Game/Blueprints/BP_Cannonball_Projectile.BP_Cannonball_Projectile_C" (Transformation|GetWorldTransform (Variables|Default|GetSpawnPoint)) "Undefined" "MultiplyWithRoot" 0 0)
          (Effects|SpawnEmitteratLocation "/Game/StarterContent/Particles/P_Explosion.P_Explosion" (Transformation|GetWorldLocation (Variables|Default|GetSpawnPoint)) "0, 0, 0" "0.500000,0.500000,0.500000")
          (Audio|PlaySoundatLocation "/Game/StarterContent/Audio/Explosion02.Explosion02" (Transformation|GetWorldLocation (Variables|Default|GetSpawnPoint)) "0, 0, 0" 1.0 1.0 0.0 0 0 0 0)
          (Default|CallOnUpdate (Variables|Default|GetAC%20Inventory))
          (if (< (.Quantity (Utilities|Struct|BreakST_Inventory_Item (.Value (Default|GetItem (Variables|Default|GetAC%20Inventory) (Variables|Default|GetCurrent))))) 1)
            (CallFunction|Drop (Variables|Default|GetCurrent))))))))

(fn ConstructionScript)

(fn ClearHand
  (bind _ac_inventory (Variables|Default|GetAC%20Inventory))
  (Default|Detach _ac_inventory)
  (Variables|/Game/Blueprints/Inventory/ActorComponents/AC_Inventory.AC_Inventory_C|SetActiveItem _ac_inventory "None")
  (Default|CallOnUpdate _ac_inventory)
  (Default|CallOnEquip _ac_inventory))

(fn Drop
  (params (ID :type Name))
  (bind _output_get (LocalVariables|SetCurrent ID))
  (if (.Success (Default|GetItem (Variables|Default|GetAC%20Inventory) _output_get))
    (Utilities|Map|Remove (Variables|/Game/Blueprints/Inventory/ActorComponents/AC_Inventory.AC_Inventory_C|GetItems (Variables|Default|GetAC%20Inventory)) (LocalVariables|GetCurrent))
    (Utilities|Unbind (Variables|/Game/Blueprints/Inventory/ActorComponents/AC_Inventory.AC_Inventory_C|GetSlots (Variables|Default|GetAC%20Inventory)) (LocalVariables|GetCurrent))
    (Default|CallOnUpdate (Variables|Default|GetAC%20Inventory))
    (CallFunction|ClearHand)))