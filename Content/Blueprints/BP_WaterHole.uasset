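; BP_WaterHole is a level hole that the player seals with a water plug, adding time to the Level 1 timer.
; On box overlap it checks for an active "waterPlug" inventory item, then once only shows the plug mesh, extends the GM_Level1 timer and flags itself plugged.
; Helper functions decrement the item's quantity in the player's ACInventory, play a drop sound, and clear the slot and hand when none remain.
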(event OnComponentBeginOverlap(Box)
  (params (OverlappedComponent :type Primitive%20Component%20Object%20Reference) (OtherActor :type Actor%20Object%20Reference) (OtherComp :type Primitive%20Component%20Object%20Reference) (OtherBodyIndex :type Integer) (bFromSweep :type Boolean) (SweepResult :type Hit%20Result%20Structure%20%28by%20ref%29))
  (if (Variables|Default|GetIsPlugAttached?)
    (Development|PrintString "plug attached")
    (else
      (bind _asfirst_person_character (Utilities|Casting|CastToFirstPersonCharacter OtherActor))
      (if (== (Variables|/Game/Blueprints/Inventory/ActorComponents/AC_Inventory.AC_Inventory_C|GetActiveItem (Variables|/Game/FirstPerson/FPSword/Blueprints/FirstPersonCharacter.FirstPersonCharacter_C|GetAC_Inventory _asfirst_person_character)) "waterPlug")
        (Utilities|FlowControl|DoOnce false
          (:Completed
            (if (not (> (Variables|Default|GetWaterPlugsAttachedAmount) 0))
              (CallFunction|UpdateInventorySlot "waterPlug")
              (bind _result (Math|Integer|IncrementInt (Variables|Default|GetWaterPlugsAttachedAmount))
                (:%20%20
                  (Variables|Default|SetWaterPlugsAttachedAmount _result)
                  (Components|StaticMesh|SetStaticMesh (Variables|Default|GetAttachMesh) (Variables|Default|GetPlug))
                  (bind _asgm_level_1 (Utilities|Casting|CastToGM_Level1 (Game|GetGameMode)))
                  (bind _output_get (Variables|Default|SetTimer (Variables|/Game/Blueprints/Gamemode/GM_Level1.GM_Level1_C|GetTimer _asgm_level_1)))
                  (Default|AddTime _output_get 6e+01)
                  (Variables|Default|SetIsPlugAttached? true))))))))))

(fn ConstructionScript)

(fn Drop
  (params (ID :type Name))
  (bind _output_get (LocalVariables|SetCurrent ID))
  (if (.Success (Default|GetItem (Variables|Default|GetAC%20Inventory) _output_get))
    (Utilities|Map|Remove (Variables|/Game/Blueprints/Inventory/ActorComponents/AC_Inventory.AC_Inventory_C|GetItems (Variables|Default|GetAC%20Inventory)) (LocalVariables|GetCurrent))
    (Utilities|Unbind (Variables|/Game/Blueprints/Inventory/ActorComponents/AC_Inventory.AC_Inventory_C|GetSlots (Variables|Default|GetAC%20Inventory)) (LocalVariables|GetCurrent))
    (Default|CallOnUpdate (Variables|Default|GetAC%20Inventory))
    (CallFunction|ClearHand)))

(fn ClearHand
  (bind _ac_inventory (Variables|Default|GetAC%20Inventory))
  (Default|Detach _ac_inventory)
  (Variables|/Game/Blueprints/Inventory/ActorComponents/AC_Inventory.AC_Inventory_C|SetActiveItem _ac_inventory "None")
  (Default|CallOnUpdate _ac_inventory)
  (Default|CallOnEquip _ac_inventory))

(fn UpdateInventorySlot
  (params (Item%20Name :type Name))
  (bind _asfirst_person_character (CallFunction|GetPlayer))
  (bind _ac_inventory (Variables|/Game/FirstPerson/FPSword/Blueprints/FirstPersonCharacter.FirstPersonCharacter_C|GetAC_Inventory _asfirst_person_character))
  (bind _activeitem (Variables|/Game/Blueprints/Inventory/ActorComponents/AC_Inventory.AC_Inventory_C|GetActiveItem _ac_inventory))
  (Variables|Default|SetAC%20Inventory _ac_inventory)
  (if (== _activeitem Item%20Name)
    (bind _output_get (Variables|Default|SetCurrent _activeitem))
    (if (.Success (Default|GetItem (Variables|Default|GetAC%20Inventory) _output_get))
      (if (.ReturnValue (Utilities|Map|Find (Variables|/Game/Blueprints/Inventory/ActorComponents/AC_Inventory.AC_Inventory_C|GetItems (Variables|Default|GetAC%20Inventory)) Item%20Name))
        (bind _result (Math|Integer|DecrementInt (.Quantity (Utilities|Struct|BreakST_Inventory_Item (.Value (Utilities|Map|Find (Variables|/Game/Blueprints/Inventory/ActorComponents/AC_Inventory.AC_Inventory_C|GetItems (Variables|Default|GetAC%20Inventory)) Item%20Name)))))
          (:%20%20
            (bind _structout (Utilities|Struct|SetmembersinST_Inventory_Item (.Value (Utilities|Map|Find (Variables|/Game/Blueprints/Inventory/ActorComponents/AC_Inventory.AC_Inventory_C|GetItems (Variables|Default|GetAC%20Inventory)) Item%20Name)) _result))
            (Utilities|Map|Add (Variables|/Game/Blueprints/Inventory/ActorComponents/AC_Inventory.AC_Inventory_C|GetItems (Variables|Default|GetAC%20Inventory)) Item%20Name _structout)
            (Audio|PlaySoundatLocation "/Engine/VREditor/Sounds/UI/Dockable_Window_Drop.Dockable_Window_Drop" (Transformation|GetActorLocation) "0, 0, 0" 1.0 1.0 0.0 0 0 0 0)
            (Default|CallOnUpdate (Variables|Default|GetAC%20Inventory))
            (if (< (.Quantity (Utilities|Struct|BreakST_Inventory_Item (.Value (Default|GetItem (Variables|Default|GetAC%20Inventory) Item%20Name)))) 1)
              (CallFunction|Drop Item%20Name)
              (return))))))))