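; Climbable ladder actor that builds itself to a set Height in both the construction script and BeginPlay.
; Side rails and collider stretch to the top, while rungs are instanced meshes spaced by CrossbarGap.
; Interaction passes the ladder to the character via SetLadderMessage and flags the first-person player as on it.
; Overlapping ColliderClimbDown clears that state, teleporting the player to TopLocation in Walking mode if the ladder's height is below TopExitPoint.
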(event OnComponentBeginOverlap(colliderclimbdown)
  (params (OverlappedComponent :type Primitive%20Component%20Object%20Reference) (OtherActor :type Actor%20Object%20Reference) (OtherComp :type Primitive%20Component%20Object%20Reference) (OtherBodyIndex :type Integer) (bFromSweep :type Boolean) (SweepResult :type Hit%20Result%20Structure%20%28by%20ref%29))
  (bind _first_person_character (Variables|Default|GetFirst%20Person%20Character))
  (if (and (< (.z (- (Transformation|GetWorldLocation (Variables|Default|Getladder%20top)) (Transformation|GetActorLocation))) (Variables|Default|GetTopExitPoint)) (Variables|/Game/FirstPerson/FPSword/Blueprints/FirstPersonCharacter.FirstPersonCharacter_C|GetIsOnLadder? (Variables|Default|GetFirst%20Person%20Character)))
    (Class|BPIClimber|SetLadder(Message) OtherActor)
    (Transformation|Teleport _first_person_character (Transformation|GetWorldLocation (Variables|Default|GetTop%20Location)) "0, 0, 0")
    (Pawn|Components|CharacterMovement|SetMovementMode (Variables|/Script/Engine.Character|GetCharacterMovement _first_person_character) "MOVE_Walking" 0)
    (Variables|/Game/FirstPerson/FPSword/Blueprints/FirstPersonCharacter.FirstPersonCharacter_C|SetIsOnLadder? _first_person_character false)))

(event Custom|Init%20Ladder
  (bind _ism_crossbar (Variables|Default|Getism%20crossbar))
  ;[0.05098 0.05098 0.05098] Initiate Ladder
  (Transformation|SetRelativeLocation (Variables|Default|Getladder%20top) (Math|Vector|MakeVector 0.0 0.0 (Variables|Default|Getheight)) false false)
  (Utilities|AdjustSideBar (Variables|Default|Getladder_L))
  (Utilities|AdjustSideBar (Variables|Default|Getladder_R))
  (Utilities|AdjustSideBar (Variables|Default|Getladder%20collider))
  (Variables|Default|Settemp_height 0.0)
  (Components|InstancedStaticMesh|ClearInstances _ism_crossbar)
  (while (< (Variables|Default|Gettemp_height) (.z (Variables|/Script/Engine.SceneComponent|GetRelativeLocation (Variables|Default|Getladder%20top))))
    (Components|InstancedStaticMesh|AddInstance _ism_crossbar (Math|Transform|MakeTransform (Math|Vector|MakeVector 0.0 0.0 (Variables|Default|Gettemp_height)) "0, 0, 0" "0.050000,0.600000,0.050000") false)
    (Variables|Default|Settemp_height (+ (Variables|Default|Gettemp_height) (Variables|Default|Getcrossbar%20gap)))))

(event EventBeginPlay
  ;[0.05098 0.05098 0.05098] BeginPlay
  (CallFunction|InitLadder)
  (bind _asfirst_person_character (Utilities|Casting|CastToFirstPersonCharacter (Game|GetPlayerCharacter 0)))
  (Variables|Default|SetFirst%20Person%20Character _asfirst_person_character))

(event EventInteraction
  (params (Character :type First%20Person%20Character%20Object%20Reference) (HitActor :type Primitive%20Component%20Object%20Reference))
  (Class|BPIClimber|SetLadder(Message) Character self)
  (Variables|/Game/FirstPerson/FPSword/Blueprints/FirstPersonCharacter.FirstPersonCharacter_C|SetIsOnLadder? (Variables|Default|GetFirst%20Person%20Character) true))

(fn ConstructionScript
  (CallFunction|InitLadder))