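; BP_Pickup is a world inventory item that the player can collect with the interaction input.
; It resolves its item from DT_Inventory by ID, or uses DropItem data if set, during construction and BeginPlay.
; The item sets the widget text and a blocking-loaded skeletal mesh, falling back to a static mesh.
; Box overlap toggles prompt and input for the local player; interacting calls PickupItemMessage on the character and destroys the actor on success.
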(event OnComponentBeginOverlap(Box)
  (params (OverlappedComponent :type Primitive%20Component%20Object%20Reference) (OtherActor :type Actor%20Object%20Reference) (OtherComp :type Primitive%20Component%20Object%20Reference) (OtherBodyIndex :type Integer) (bFromSweep :type Boolean) (SweepResult :type Hit%20Result%20Structure%20%28by%20ref%29))
  (if (== (CallFunction|GetPlayer) OtherActor)
    (Utilities|IsPlayer (CallFunction|GetPlayer)
      (:true
        (Rendering|SetVisibility (Variables|Default|GetWidget) true false)
        (Input|EnableInput (Game|GetPlayerController 0))
        (Variables|Default|SetCharacter (CallFunction|GetPlayer))))))

(event OnComponentEndOverlap(Box)
  (params (OverlappedComponent :type Primitive%20Component%20Object%20Reference) (OtherActor :type Actor%20Object%20Reference) (OtherComp :type Primitive%20Component%20Object%20Reference) (OtherBodyIndex :type Integer))
  (bind _ascharacter (Utilities|Casting|CastToCharacter OtherActor))
  (Utilities|IsPlayer _ascharacter
    (:true
      (Rendering|SetVisibility (Variables|Default|GetWidget) false false)
      (Input|DisableInput (Game|GetPlayerController 0)))))

(event Custom|Update
  (bind _item (Variables|Default|GetItem))
  (bind (_displayname _thumbnail _pickupmesh _pickupmeshstatic) (Utilities|Struct|BreakST_Inventory_Item _item))
  (bind _aswb_interact (Utilities|Casting|CastToWB_Interact (UserInterface|GetWidget (Variables|Default|GetWidget))))
  (Rendering|Components|TextRender|SetText (Variables|/Game/Blueprints/Inventory/Widgets/WB_Interact.WB_Interact_C|GetTEXT _aswb_interact) _displayname)
  (bind _returnvalue (Utilities|LoadAssetBlocking _pickupmesh))
  (bind _asskeletal_mesh (Utilities|Casting|CastToSkeletalMesh _returnvalue)
    (:then
      (Components|SkeletalMesh|SetSkeletalMeshAsset (Variables|Default|GetSkeletalMesh) _asskeletal_mesh))
    (:CastFailed
      (bind _returnvalue_2 (Utilities|LoadAssetBlocking _pickupmeshstatic))
      (bind _asstatic_mesh (Utilities|Casting|CastToStaticMesh _returnvalue_2))
      (Components|StaticMesh|SetStaticMesh (Variables|Default|GetStaticMesh) _asstatic_mesh))))

(event Input|EnhancedActionEvents|EnhancedInputActionIA_Interaction
  (params (ActionValue :type Boolean) (ElapsedSeconds :type Float%20%28double-precision%29) (TriggeredSeconds :type Float%20%28double-precision%29) (InputAction :type Input%20Action%20Object%20Reference :default "/Game/FirstPerson/Input/Actions/IA_Interaction.IA_Interaction"))
  (:Started
    (bind _success (Class|BPIInventory|PickupItem(Message) (Variables|Default|GetCharacter) (Variables|Default|GetID) (Variables|Default|GetItem)))
    (if _success
      (Actor|DestroyActor))))

(event EventBeginPlay
  (CallFunction|GetID))

(fn ConstructionScript
  (CallFunction|GetID))

(fn GetID
  (bind _returnvalue (Utilities|GetDataTableRow "/Game/Blueprints/Inventory/Data/Datatables/DT_Inventory.DT_Inventory" (Variables|Default|GetID))
    (:then
      (bind _output_get (Variables|Default|SetItem (select (!= (.ID (Utilities|Struct|BreakST_Inventory_Item (Variables|Default|GetDropItem))) "") (Variables|Default|GetDropItem) _returnvalue)))
      (CallFunction|Update)
      (return _output_get))))