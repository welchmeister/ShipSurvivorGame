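; BP_Axe is an inventory axe whose Attack event strikes breakable objects in front of the player.
; Attack runs a short visibility line trace forward from the first-person camera, ignoring the axe itself.
; If the hit actor implements BPI_Breakable_Axe, it waits half a second, spawns FS_Impact at the impact point and sends that actor a RemoveWidgets message.
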(event Custom|Attack
  (bind _asfirst_person_character (CallFunction|GetPlayer))
  (bind _firstpersoncamera (Variables|/Game/FirstPerson/FPSword/Blueprints/FirstPersonCharacter.FirstPersonCharacter_C|GetFirstPersonCamera _asfirst_person_character))
  (bind _returnvalue (Transformation|GetWorldLocation _firstpersoncamera))
  (bind (_outhit _returnvalue_2) (Collision|LineTraceByChannel _returnvalue (+ _returnvalue (* (Math|Vector|GetForwardVector _firstpersoncamera) 1.1e+02)) "TraceTypeQuery1" false (Utilities|Array|MakeArray self) "None"))
  (if _returnvalue_2
    (if (Utilities|DoesObjectImplementInterface (.HitActor (Collision|BreakHitResult _outhit)) "/Game/Blueprints/Interfaces/BPI_Breakable_Axe.BPI_Breakable_Axe_C")
      (Utilities|FlowControl|Delay 0.5)
      (Game|SpawnActorfromClass "/Game/Blueprints/BreakableJug/FS_Impact.FS_Impact_C" (Math|Transform|MakeTransform (.ImpactPoint (Collision|BreakHitResult _outhit)) "0, 0, 0" "1.000000,1.000000,1.000000") "Undefined" "MultiplyWithRoot" 0 0)
      (Class|BPIBreakableAxe|RemoveWidgets(Message) (.HitActor (Collision|BreakHitResult _outhit))))))

(fn ConstructionScript)