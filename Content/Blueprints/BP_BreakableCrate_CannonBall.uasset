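; Crate Blueprint that reacts to cannonball hits and shows an instruction widget when the player is nearby.
; Overlap on Box from any actor implementing BPI_Cannonball spawns an explosion and collapse sound, disables both boxes' collision responses and hides the widget.
; InteractBox overlaps toggle that widget for the player.
; The graph neither destroys the actor nor hides its mesh.
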(event OnComponentBeginOverlap(Box)
  (params (OverlappedComponent :type Primitive%20Component%20Object%20Reference) (OtherActor :type Actor%20Object%20Reference) (OtherComp :type Primitive%20Component%20Object%20Reference) (OtherBodyIndex :type Integer) (bFromSweep :type Boolean) (SweepResult :type Hit%20Result%20Structure%20%28by%20ref%29))
  (if (Utilities|DoesObjectImplementInterface OtherActor "/Game/Blueprints/Interfaces/BPI_Cannonball.BPI_Cannonball_C")
    (Effects|SpawnEmitteratLocation "/Game/StarterContent/Particles/P_Explosion.P_Explosion" (Transformation|GetActorLocation))
    (Audio|PlaySoundatLocation "/Game/StarterContent/Audio/Collapse02.Collapse02" (Transformation|GetActorLocation) "0, 0, 0" 1.0 1.0 0.0 0 0 0 0)
    (Collision|SetCollisionResponsetoAllChannels (Variables|Default|GetBox) "ECR_Ignore")
    (Collision|SetCollisionResponsetoAllChannels (Variables|Default|GetInteractBox) "ECR_Ignore")
    (Rendering|SetVisibility (Variables|Default|GetInstructionWidget) false false)))

(event OnComponentBeginOverlap(InteractBox)
  (params (OverlappedComponent :type Primitive%20Component%20Object%20Reference) (OtherActor :type Actor%20Object%20Reference) (OtherComp :type Primitive%20Component%20Object%20Reference) (OtherBodyIndex :type Integer) (bFromSweep :type Boolean) (SweepResult :type Hit%20Result%20Structure%20%28by%20ref%29))
  (if (== OtherActor (CallFunction|GetPlayer))
    (Rendering|SetVisibility (Variables|Default|GetInstructionWidget) true false)))

(event OnComponentEndOverlap(InteractBox)
  (params (OverlappedComponent :type Primitive%20Component%20Object%20Reference) (OtherActor :type Actor%20Object%20Reference) (OtherComp :type Primitive%20Component%20Object%20Reference) (OtherBodyIndex :type Integer))
  (if (== OtherActor (CallFunction|GetPlayer))
    (Rendering|SetVisibility (Variables|Default|GetInstructionWidget) false false)))

(fn ConstructionScript)