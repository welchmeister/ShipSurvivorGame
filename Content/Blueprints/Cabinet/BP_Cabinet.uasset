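; BP_Cabinet is a cabinet with a door that swings open and closed when interacted with.
; InteractFurniture compares the hit component's display name to the door's, then a FlipFlop alternates between playing the timeline forward and in reverse.
; The timeline alpha lerps the door's yaw through a quarter turn, and both directions play the same drawer-close sound at the cabinet's location.
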(event EventInteractFurniture
  (params (HitComponent :type Primitive%20Component%20Object%20Reference))
  (bind _returnvalue (Transformation|GetActorLocation))
  (if (Utilities|Enum|Equal(Enum) (Utilities|GetDisplayName HitComponent) "BP_Cabinet.Door CabinetDoor")
    (Utilities|FlowControl|FlipFlop
      (:A
        (Audio|PlaySoundatLocation "/Game/Meshes/PuzzleMeshes/Audio/DoorsAndFurnitures/DrawerClose02.DrawerClose02" _returnvalue "0, 0, 0" 1.0 1.0 0.0 0 0 0 0)
        (bind _alpha (Timeline|Timeline PlayFromStart)
          (:Update
            (Transformation|SetRelativeRotation (Variables|Default|GetDoor) (Math|Rotator|MakeRotator 0.0 0.0 (Math|Float|Lerp 0.0 9e+01 _alpha)) false false))))
      (:B
        (Audio|PlaySoundatLocation "/Game/Meshes/PuzzleMeshes/Audio/DoorsAndFurnitures/DrawerClose02.DrawerClose02" _returnvalue "0, 0, 0" 1.0 1.0 0.0 0 0 0 0)
        (Timeline|Timeline ReverseFromEnd)))))

(fn ConstructionScript)