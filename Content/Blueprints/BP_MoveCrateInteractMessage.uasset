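; Interactable prompt for a movable crate that the player shifts with a crowbar to clear a blocked spot.
; An overlap box shows the interact and instruction widgets to the first-person character until the crate is moved.
; Interaction checks the player's active inventory item for the crowbar, then triggers MoveCrate on MovingCrate, hides both widgets and disables the blocking box's collision.
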(event OnComponentBeginOverlap(OverlapBox)
  (params (OverlappedComponent :type Primitive%20Component%20Object%20Reference) (OtherActor :type Actor%20Object%20Reference) (OtherComp :type Primitive%20Component%20Object%20Reference) (OtherBodyIndex :type Integer) (bFromSweep :type Boolean) (SweepResult :type Hit%20Result%20Structure%20%28by%20ref%29))
  ;[1 1 1] Box Overlap Events to display widget instructions for door.
  (if (Variables|Default|GetIsCratedMoved?)
    (Rendering|SetVisibility (Variables|Default|GetInteractWidget) false false)
    (Rendering|SetVisibility (Variables|Default|GetInstructionsWidget) false false)
    (else
      (Utilities|Casting|CastToFirstPersonCharacter OtherActor)
      (Rendering|SetVisibility (Variables|Default|GetInteractWidget) true false)
      (Rendering|SetVisibility (Variables|Default|GetInstructionsWidget) true false))))

(event OnComponentEndOverlap(OverlapBox)
  (params (OverlappedComponent :type Primitive%20Component%20Object%20Reference) (OtherActor :type Actor%20Object%20Reference) (OtherComp :type Primitive%20Component%20Object%20Reference) (OtherBodyIndex :type Integer))
  ;[1 1 1] Box Overlap Events to display widget instructions for door.
  (if (not (Variables|Default|GetIsCratedMoved?))
    (Utilities|Casting|CastToFirstPersonCharacter OtherActor)
    (Rendering|SetVisibility (Variables|Default|GetInteractWidget) false false)
    (Rendering|SetVisibility (Variables|Default|GetInstructionsWidget) false false)))

(event EventInteraction
  (params (Character :type First%20Person%20Character%20Object%20Reference) (HitActor :type Primitive%20Component%20Object%20Reference))
  (if (== (Variables|/Game/Blueprints/Inventory/ActorComponents/AC_Inventory.AC_Inventory_C|GetActiveItem (Variables|/Game/FirstPerson/FPSword/Blueprints/FirstPersonCharacter.FirstPersonCharacter_C|GetAC_Inventory (CallFunction|GetPlayer))) "crowbar")
    (Variables|Default|SetIsCratedMoved? true)
    (Default|MoveCrate (Variables|Default|GetMovingCrate))
    (Rendering|SetVisibility (Variables|Default|GetInteractWidget) false false)
    (Rendering|SetVisibility (Variables|Default|GetInstructionsWidget) false false)
    (Collision|SetCollisionEnabled (Variables|Default|GetBlockingBox) "NoCollision")))

(fn ConstructionScript)